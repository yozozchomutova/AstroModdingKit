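; Seeder machine from the HungerSystem mod that spins a rotary part while it consumes an Organic item from its slot.
; On BeginPlay it binds the slot's set-item delegate to store the placed item and shows an Organic resource-request indicator.
; While an item is stored, Tick rotates the rotary and drains the item's fullness over time.
; When drained, the item is destroyed, the reference cleared and the indicator restored; no seed output occurs here.
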(event `self.ReceiveBeginPlay`
  (add `SlotDelegates.OnSetItem` (`SlotsComponent.GetSlotDelegates` (`ChildSlotComponent.MakeReference` (`self.OrganicSlot`))) (delegate `Placed In Slot`))
  (`self.RefreshIndicator`))

(event `Placed In Slot`
  (params (Item :type "PhysicalItem Object Reference"))
  (set `self.OrganicItem` Item))

(event `self.ReceiveTick`
  (params (DeltaSeconds :type "Float (single-precision)"))
  (bind _itemcomponent (`PhysicalItem.ItemComponent` (`self.OrganicItem`)))
  (bind _returnvalue (`KismetMathLibrary.FMax` (- (`ItemComponent.GetFullness` _itemcomponent) (* DeltaSeconds 0.2))))
  (if (not (== (`self.OrganicItem`) null))
    (`SceneComponent.K2_AddLocalRotation` (`self.Rotary`) (`KismetMathLibrary.MakeRotator` 0.0 0.0 (* DeltaSeconds 30.0)) false false)
    (`ItemComponent.SetAmountUsingFullness` _itemcomponent _returnvalue false)
    (if (<= _returnvalue 0.0)
      (`SlotsComponent.DestroySlotItem` (`self.SlotsComponent`) (`ChildSlotComponent.MakeReference` (`self.OrganicSlot`)))
      (set `self.OrganicItem` null)
      (`self.RefreshIndicator`))))

(fn `GetBodySlotLegacy`
  (returns (ReturnValue :type "ChildSlotComponent Object Reference"))
  (return (`self.BodySlot`)))

(fn `RefreshIndicator`
  (`SlotsComponent.SlotAttemptToPushIndicatorIntoSpecificSubslot` (`ChildSlotComponent.MakeReference` (`self.OrganicSlot`)) 0 (make `SlotIndicatorDefinition` "/Game/Items/ItemTypes/Minables/Organic.Organic_C")))

(fn `UserConstructionScript`)