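; Cargo launch pad for the SpaceStorage mod that loads and unloads resources for a docked rocket and receives delivery pods from station storage.
; Rocket input and output run through slot delegates, with Tick animating item drain and fill.
; The control panel UI receives dock events, and unloading grants research points and destroys empty pods.
; Tick also eases loader tower and pin bones in staged order, while power updates drive gauge materials.
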(event `OnItemPlacedInputSlot`
  (params (Item :type "PhysicalItem Object Reference"))
  (bind _success (`/Game/Mods/Yzch/SpaceStorage/PhysicalCargoRocket.InputResource` (`self.ConnectedRocket`) Item))
  (if _success
    (`self.EraseResource` (`self.GetInputSlot`) Item)))

(event `UpdateItemSlotsEvent`
  (`self.SetInputSlotTooltipIndicator` (not (`/Game/Mods/Yzch/SpaceStorage/PhysicalCargoRocket.UnloadingMode` (`self.ConnectedRocket`)))))

(event `OnRocketConnectedEvent`
  (bind _connectedrocket (`self.ConnectedRocket`))
  (bind _resourcecurrentamount (`/Game/Mods/Yzch/SpaceStorage/PhysicalCargoRocket.ResourceCurrentAmount` _connectedrocket))
  (if (and (`self.RocketIsOnGround`) (`self.RocketIsUnloading`)) :!label _label
    (bind (_success _resource) (`/Game/Mods/Yzch/SpaceStorage/PhysicalCargoRocket.OutputResource` (`self.ConnectedRocket`)))
    (if _success
      (`self.SpawnResource` (`self.GetOutputSlot`) _resource))
    (`ResearchSystem.AuthorityGrantResearchPoints` _resourcecurrentamount)
    (if (and (`/Game/Mods/Yzch/SpaceStorage/PhysicalCargoRocket.IsDeliveryPod` _connectedrocket) (<= _resourcecurrentamount 0))
      (`/Game/Mods/Yzch/SpaceStorage/PhysicalCargoRocket.DestroyRocket` (`self.ConnectedRocket`)))))

(event `UpdateOutputSlotEvent`
  (params (Item :type "PhysicalItem Object Reference"))
  (goto _label))

(event `self.ReceiveBeginPlay`
  (`|ExecutionSequence`
    (:`then_0`
      (`|ExecutionSequence`
        (:`then_0`
          (bind _returnvalue (`KismetMaterialLibrary.CreateDynamicMaterialInstance` "/Game/Mods/Yzch/SpaceStorage/Materials/RedLights.RedLights"))
          (set `self.RedLightMatDynamicInstance` _returnvalue))
        (:`then_1`
          (bind _aspad_control_panel (cast `/Game/Mods/Yzch/SpaceStorage/PadControlPanel` (`ChildActorComponent.ChildActor` (`self.PadControlPanel`))))
          (bind _output_get (set `self.ControlPanel` _aspad_control_panel))
          (bind _padcontrolui (`/Game/Mods/Yzch/SpaceStorage/PadControlPanel.GetPadControlUIRef` _output_get))
          (set `/Game/Mods/Yzch/SpaceStorage/PadControlUI.CargoShipLaunchPad` self _padcontrolui)
          (add `/Game/Mods/Yzch/SpaceStorage/PadControlUI.UpdateItemSlots` _padcontrolui (delegate `UpdateItemSlotsEvent`))
          (add `SlotDelegates.OnSetItem` (`SlotsComponent.GetSlotDelegates` (`self.GetInputSlot`)) (delegate `OnItemPlacedInputSlot`))
          (add `SlotDelegates.OnReleaseItem` (`SlotsComponent.GetSlotDelegates` (`self.GetOutputSlot`)) (delegate `UpdateOutputSlotEvent`)))
        (:`then_2`
          (bind _assm_cargo_rocket_bp (cast `/Game/Mods/Yzch/SpaceStorage/SmCargoRocket_BP` (`SlotsComponent.GetSlotItem` (`SlotsComponent.MakeReference` (`self.SlotsComponent`) "RocketSlot"))))
          (`self.OnRocketConnect` _assm_cargo_rocket_bp))
        (:`then_3`
          (bind (_direction _materialintensity _lightintensity) (`Timeline|Lighting` :!via `PlayFromStart`)
            (:`Update`
              (`|ExecutionSequence`
                (:`then_0`
                  (`MaterialInstanceDynamic.SetScalarParameterValue` (`self.RedLightMatDynamicInstance`) "Intensity" (* _materialintensity 100.0)))
                (:`then_1`
                  (`LightComponent.SetIntensity` (`self.RedLights`) (* _lightintensity 40000.0)))))))
        (:`then_4`
          (`/Game/Mods/Yzch/SpaceStorage/PadControlPanel.OnBeginLaunchpad` (`self.ControlPanel`))
          (bind _returnvalue_2 (`PrimitiveComponent.CreateDynamicMaterialInstance` (`self.StaticMeshComponent`) 1 "/Game/Materials/modules/MI_palette_exo_dynamic_fillbar_power_lights_only.MI_palette_exo_dynamic_fillbar_power_lights_only" "None"))
          (set `self.PowerGaugesMat` _returnvalue_2))))
    (:`then_1`
      (bind _logger (`/Game/Mods/localcc/DebugConsole/ConsoleLogging.GetLogger` :!label _label_2))
      (bind (_consumerdemandfulfilmentratio _generationratio _surplusratio) (break `StreamingPowerNodeVisualizationData` (stale `self.ActorStreamingPowerNode.OnUpdatePowerVisualization` VisualizationData)))
      (`/Game/Mods/localcc/DebugConsole/ConsoleWidget.AddLogMessage` _logger (`KismetStringLibrary.Concat_StrStr` (`KismetStringLibrary.Conv_DoubleToString` _consumerdemandfulfilmentratio) " / " (`KismetStringLibrary.Conv_DoubleToString` _generationratio) " / " (`KismetStringLibrary.Conv_DoubleToString` _surplusratio)) "NewEnumerator0")
      (`MaterialInstanceDynamic.SetScalarParameterValue` (`self.PowerGaugesMat`) "ConsumptionGaugePercent" _consumerdemandfulfilmentratio)
      (`MaterialInstanceDynamic.SetScalarParameterValue` (`self.PowerGaugesMat`) "GenerationGaugePercent" _generationratio)
      (`MaterialInstanceDynamic.SetScalarParameterValue` (`self.PowerGaugesMat`) "OnOffSwitch" (/ (`KismetMathLibrary.Conv_BoolToDouble` (or (!= _consumerdemandfulfilmentratio 0.0) (!= _generationratio 0.0))) 4.0)))))

(event `self.ReceiveTick`
  (params (DeltaSeconds :type "Float (single-precision)"))
  (bind _eraseinputresource_fullness (`self.EraseInputResource_Fullness`))
  (bind _spawnoutputresource_fullness (`self.SpawnOutputResource_Fullness`))
  (bind _itemcomponent (`PhysicalItem.ItemComponent` (`SlotsComponent.GetSlotItem` (`self.GetOutputSlot`))))
  (`|ExecutionSequence`
    (:`then_0`
      (if (`self.BonesMoving`)
        (`self.UpdateBones` DeltaSeconds (not (== (`self.ConnectedRocket`) null)))))
    (:`then_1`
      (if (> (`self.EraseInputResource_Fullness`) 0.0)
        (bind _output_get (set `self.EraseInputResource_Fullness` (- (stale _output_get) (* DeltaSeconds 0.8))))
        (if (> _eraseinputresource_fullness 0.0)
          (`ItemComponent.SetAmountUsingFullness` (`self.EraseInputResource_Component`) _eraseinputresource_fullness false)
          (else
            (`SlotsComponent.DestroySlotItem` (`self.GetInputSlot`))
            (set `ChildSlotComponent.Unclickable` false (`self.InputItem`))))))
    (:`then_2`
      (bind _logger (`/Game/Mods/localcc/DebugConsole/ConsoleLogging.GetLogger`)))
    (:`then_3`
      (if (< (`self.SpawnOutputResource_Fullness`) 1.0)
        (bind _output_get_2 (set `self.SpawnOutputResource_Fullness` (+ (stale _output_get_2) (* DeltaSeconds 0.5))))
        (bind _physical_item (`/Game/Mods/Yzch/SpaceStorage/MoreSlotFunctions.GetSlotItem` (`self.OutputItem`)))
        (if (== _physical_item null)
          _
          (elif (< _spawnoutputresource_fullness 1.0)
            (bind _returnvalue (`ItemComponent.SetAmountUsingFullness` _itemcomponent _spawnoutputresource_fullness false))
            (else
              (`ItemComponent.SetAmountUsingFullness` _itemcomponent 1.0 false)
              (if (not (> (`/Game/Mods/Yzch/SpaceStorage/PhysicalCargoRocket.ResourceCurrentAmount` (`self.ConnectedRocket`)) 0))
                (set `/Game/Mods/Yzch/SpaceStorage/PhysicalCargoRocket.UnloadingMode` false (`self.ConnectedRocket`))))))))))

(event `self.PickedUpFromWorld`
  ;[1 0.02273 0] Collision when slotted
)

(event `self.StartInWorld`
  ;[1 0.02273 0] Collision when slotted
)

(event `self.PlacedInSlot`
  (params (Slot :type "SlotReference Structure") (FromTool :type Boolean) (SlottedDuringInitialization :type Boolean))
  ;[1 0.02273 0] Collision when slotted
)

(event `self.ActorStreamingPowerNode.OnUpdatePowerVisualization`
  (params (VisualizationData :type "StreamingPowerNodeVisualizationData Structure (by ref)"))
  (goto _label_2))

(fn `EraseResource`
  (params (`Input Slot` :type "SlotReference Structure") (Resource :type "PhysicalItem Object Reference"))
  (set `ChildSlotComponent.Unclickable` true (`self.InputItem`))
  (set `self.EraseInputResource_Fullness` 1.0)
  (set `self.EraseInputResource_Component` (`PhysicalItem.ItemComponent` Resource)))

(fn `GetBodySlotLegacy`
  (returns (ReturnValue :type "ChildSlotComponent Object Reference"))
  (return (`self.BodySlot`)))

(fn `GetResourcesAreBeingDelivered`
  (returns (`Being Delivered` :type Boolean))
  (return (== (`GameplayStatics.GetObjectClass` (`SlotsComponent.GetSlotPrimaryItem` (`ChildSlotComponent.MakeReference` (`self.RocketSlot`)))) "/Game/Mods/Yzch/SpaceStorage/CargoResourcePod_BP.CargoResourcePod_BP_C")))

(fn `OnRocketConnect`
  (params (CargoRocket :type "/Game/Mods/Yzch/SpaceStorage/PhysicalCargoRocket Object Reference"))
  (bind _output_get (set `self.ConnectedRocket` CargoRocket))
  (set `/Game/Mods/Yzch/SpaceStorage/PhysicalCargoRocket.ConnectedPad` self CargoRocket)
  (set `self.BonesMoving` true)
  (`/Game/Mods/Yzch/SpaceStorage/PadControlUI.OnRocketConnected` (`/Game/Mods/Yzch/SpaceStorage/PadControlPanel.PadControlUIRef` (`self.ControlPanel`)) _output_get)
  (`self.OnRocketConnectedEvent`))

(fn `OnRocketDisconnect`
  (params (CargoRocket :type "/Game/Mods/Yzch/SpaceStorage/PhysicalCargoRocket Object Reference"))
  (set `self.ConnectedRocket` null)
  (set `self.BonesMoving` true)
  (`/Game/Mods/Yzch/SpaceStorage/PadControlUI.OnRocketDisconnected` (`/Game/Mods/Yzch/SpaceStorage/PadControlPanel.PadControlUIRef` (`self.ControlPanel`))))

(fn `RequestStationResourceDelivery`
  (params (ResourceType :type "ItemType Class Reference") (Amount :type Integer))
  (bind _space_station (`/Game/Mods/Yzch/SpaceStorage/SpaceStation/SpaceStationSingleton.GetSingleton`))
  (`/Game/Mods/Yzch/SpaceStorage/SpaceStation/SpaceStation.RemoveResourcesFromStorage` _space_station ResourceType Amount)
  (bind _returnvalue (`SlotsComponent.SpawnActorInSlot` (`self.SlotsComponent`) (`ChildSlotComponent.MakeReference` (`self.RocketSlot`)) "/Game/Mods/Yzch/SpaceStorage/CargoResourcePod_BP.CargoResourcePod_BP_C"))
  (bind _ascargo_resource_pod_bp (cast `/Game/Mods/Yzch/SpaceStorage/CargoResourcePod_BP` _returnvalue))
  (set `/Game/Mods/Yzch/SpaceStorage/PhysicalCargoRocket.CurrentResource` ResourceType _ascargo_resource_pod_bp)
  (set `/Game/Mods/Yzch/SpaceStorage/PhysicalCargoRocket.ResourceCurrentAmount` Amount _ascargo_resource_pod_bp)
  (`ResearchSystem.AuthorityGrantResearchPoints` Amount)
  (set `/Game/Mods/Yzch/SpaceStorage/PhysicalCargoRocket.UnloadingMode` true _ascargo_resource_pod_bp)
  (`self.OnRocketConnect` _ascargo_resource_pod_bp)
  (`/Game/Mods/Yzch/SpaceStorage/PhysicalCargoRocket.TryLaunch` _ascargo_resource_pod_bp))

(fn `SetInputSlotTooltipIndicator`
  (params (Visible :type Boolean))
  (bind _slot_reference (`self.GetInputSlot`))
  (bind _currentresource (`/Game/Mods/Yzch/SpaceStorage/PhysicalCargoRocket.CurrentResource` (`self.ConnectedRocket`)))
  (if (== null _currentresource)
    (`SlotsComponent.SlotDestroyIndicators` _slot_reference :!label _label)
    (elif Visible
      (`SlotsComponent.SlotAttemptToPushIndicatorIntoSpecificSubslot` _slot_reference 0 (make `SlotIndicatorDefinition` _currentresource))
      (else
        (goto _label)))))

(fn `SpawnResource`
  (params (`Output Slot` :type "SlotReference Structure") (Resource :type "ItemType Class Reference"))
  (set `self.SpawnOutputResource_Fullness` 0.0)
  (`SlotsComponent.SpawnItemTypeInSlot` (`ChildSlotComponent.MakeReference` (`self.OutputItem`)) Resource)
  (set `self.SpawnOutputResource_Component` null))

(fn `UpdateBoneLocation`
  (params (`Bone Name` :type Name) (`Axis ID` :type Integer) (`New Location` :type "Float (double-precision)"))
  (bind _returnvalue (`PoseableMeshComponent.GetBoneLocationByName` (`self.LoaderMesh`) `Bone Name` "ComponentSpace"))
  (switch `int` `Axis ID`
    (:`0`
      (bind _x (.x _returnvalue))
      (bind _y (.y _returnvalue))
      (bind _z (.z _returnvalue))
      (`PoseableMeshComponent.SetBoneLocationByName` (`self.LoaderMesh`) `Bone Name` (`KismetMathLibrary.MakeVector` `New Location` _y _z) "ComponentSpace"))
    (:`1`
      (`PoseableMeshComponent.SetBoneLocationByName` (`self.LoaderMesh`) `Bone Name` (`KismetMathLibrary.MakeVector` _x `New Location` _z) "ComponentSpace"))
    (:`2`
      (`PoseableMeshComponent.SetBoneLocationByName` (`self.LoaderMesh`) `Bone Name` (`KismetMathLibrary.MakeVector` _x _y `New Location`) "ComponentSpace"))))

(fn `UpdateBones`
  (params (`Delta Seconds` :type "Float (double-precision)") (`Rocket Connected` :type Boolean))
  (locals (ChangeRate :type "Float (double-precision)") (`Rocket Connected_` :type Boolean))
  (bind _redlights (`self.RedLights`))
  (bind (_relativelocation_x _relativelocation_y) (`KismetMathLibrary.BreakVector` (`SceneComponent.RelativeLocation` _redlights)))
  (set `local.ChangeRate` (* `Delta Seconds` 3.0))
  (bind _output_get (set `local.Rocket Connected_` `Rocket Connected`))
  (`|ExecutionSequence`
    (:`then_0`
      (if (and _output_get (`self.RocketIsOnGround`))
        (`|ExecutionSequence`
          (:`then_0`
            (bind _close_to_target (`self.UpdateBoneValues` (`self.SideTower_OffBase`) (`self.SideTower_OffCurrent`) (`self.SideTower_OffMax`) (`local.ChangeRate`) (`self.RocketIsNotDeliveryPod`)))
            (if _close_to_target
              (bind _close_to_target_2 (`self.UpdateBoneValues` (`self.SidePins_OffBase`) (`self.SidePins_OffCurrent`) (`self.SidePins_OffMax`) (`local.ChangeRate`) (`self.RocketIsNotDeliveryPod`)))))
          (:`then_1`
            (bind _close_to_target_3 (`self.UpdateBoneValues` (`self.BackTower_OffBase`) (`self.BackTower_OffCurrent`) (`self.BackTower_OffMax`) (`local.ChangeRate`) (`local.Rocket Connected_`)))
            (if _close_to_target_3
              (bind _close_to_target_4 (`self.UpdateBoneValues` (`self.BackPins_OffBase`) (`self.BackPins_OffCurrent`) (`self.BackPins_OffMax`) (`local.ChangeRate`) (`local.Rocket Connected_`)))))
          (:`then_2`
            (bind _close_to_target_5 (`self.UpdateBoneValues` (`self.TopTower_OffBase`) (`self.TopTower_OffCurrent`) (`/Game/Mods/Yzch/SpaceStorage/PhysicalCargoRocket.UpperPinHeight` (`self.ConnectedRocket`)) (`local.ChangeRate`) (`self.RocketIsNotDeliveryPod`)))
            (if _close_to_target_5
              (bind _close_to_target_6 (`self.UpdateBoneValues` (`self.TopPins_OffBase`) (`self.TopPins_OffCurrent`) (`self.TopPins_OffMax`) (`local.ChangeRate`) (`self.RocketIsNotDeliveryPod`)))
              (if (and _close_to_target_2 _close_to_target_4 _close_to_target_6)
                (set `self.BonesMoving` false)))))
        (else
          (`|ExecutionSequence`
            (:`then_0`
              (bind _close_to_target_7 (`self.UpdateBoneValues` (`self.SidePins_OffBase`) (`self.SidePins_OffCurrent`) (`self.SidePins_OffMax`) (`local.ChangeRate`) (`self.RocketIsNotDeliveryPod`)))
              (if _close_to_target_7
                (bind _close_to_target_8 (`self.UpdateBoneValues` (`self.SideTower_OffBase`) (`self.SideTower_OffCurrent`) (`self.SideTower_OffMax`) (`local.ChangeRate`) (`self.RocketIsNotDeliveryPod`)))))
            (:`then_1`
              (bind _close_to_target_9 (`self.UpdateBoneValues` (`self.BackPins_OffBase`) (`self.BackPins_OffCurrent`) (`self.BackPins_OffMax`) (`local.ChangeRate`) (`local.Rocket Connected_`)))
              (if _close_to_target_9
                (bind _close_to_target_10 (`self.UpdateBoneValues` (`self.BackTower_OffBase`) (`self.BackTower_OffCurrent`) (`self.BackTower_OffMax`) (`local.ChangeRate`) (`local.Rocket Connected_`)))))
            (:`then_2`
              (bind _close_to_target_11 (`self.UpdateBoneValues` (`self.TopPins_OffBase`) (`self.TopPins_OffCurrent`) (`self.TopPins_OffMax`) (`local.ChangeRate`) (`self.RocketIsNotDeliveryPod`)))
              (if _close_to_target_11
                (bind _close_to_target_12 (`self.UpdateBoneValues` (`self.TopTower_OffBase`) (`self.TopTower_OffCurrent`) (`self.TopTower_OffMax`) (`local.ChangeRate`) (`self.RocketIsNotDeliveryPod`)))
                (if (and _close_to_target_8 _close_to_target_10 _close_to_target_12)
                  (set `self.BonesMoving` false))))))))
    (:`then_1`
      (`self.UpdateBoneLocation` "SideTower" 2 (`self.SideTower_OffCurrent`))
      (`self.UpdateBoneLocation` "TopTower" 2 (`self.TopTower_OffCurrent`))
      (`self.UpdateBoneLocation` "BackTower" 2 (`self.BackTower_OffCurrent`))
      (`self.UpdateBoneLocation` "SidePins" 0 (`self.SidePins_OffCurrent`))
      (`self.UpdateBoneLocation` "TopPins" 0 (`self.TopPins_OffCurrent`))
      (`self.UpdateBoneLocation` "BackPins" 1 (`self.BackPins_OffCurrent`))
      (`SceneComponent.K2_SetRelativeLocation` _redlights (`KismetMathLibrary.MakeVector` _relativelocation_x _relativelocation_y (+ 600.0 (`self.TopTower_OffCurrent`))) false false))))

(fn `UpdateBoneValues`
  (params (OffBase :type "Float (double-precision)") (OffCurrent :type "Float (double-precision) (by ref)") (OffMax :type "Float (double-precision)") (`Change Rate` :type "Float (double-precision)") (`Rocket Connected` :type Boolean))
  (returns (`Close To Target` :type Boolean))
  (bind _returnvalue (- (select `bool` `Rocket Connected` :`false` OffBase :`true` OffMax) OffCurrent))
  (`|VariableSetRef` OffCurrent (+ (* _returnvalue `Change Rate`) OffCurrent))
  (return (<= (`KismetMathLibrary.Abs` _returnvalue) 15.0)))

(fn `UserConstructionScript`)