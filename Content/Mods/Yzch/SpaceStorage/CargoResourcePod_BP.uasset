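; Cargo resource pod rocket Blueprint that animates a launch flight, then returns the rocket and grants research points.
; On launch, DescendTimeline curves offset the static mesh along the launch location's up and forward vectors and pitch it from the launch rotation.
; The playback position is stored each update, so BeginPlay resumes an unfinished flight from that timestamp.
; It also exposes RocketBodySlot through GetBodySlotLegacy.
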(event `self.OnLaunch`
  (bind _launchworldlocation (`self.LaunchWorldLocation`))
  (`parent.OnLaunch`)
  (set `self.LaunchAnimTimestamp` 0.0)
  (`|ExecutionSequence` :!label _label
    (:`then_0`
      (bind (_direction _rotationfloat _positionvertical _positionhorizontal) (`Timeline|Descend Timeline` :`NewTime` (`self.LaunchAnimTimestamp`) :!via `SetNewTime` :!label _label_2)
        (:`Update`
          (set `self.LaunchAnimTimestamp` (`TimelineComponent.GetPlaybackPosition` (`self.Descend Timeline`)))
          (`SceneComponent.K2_SetWorldLocationAndRotation` (`self.StaticMeshComponent`) (+ (`SceneComponent.K2_GetComponentLocation` (`self.LaunchWorldLocation`)) (* (`SceneComponent.GetUpVector` _launchworldlocation) (* _positionvertical 20000.0)) (* (`SceneComponent.GetForwardVector` _launchworldlocation) (* _positionhorizontal -3800.0))) (`KismetMathLibrary.MakeRotator` (.roll (`self.LaunchWorldRotation`)) (+ (.pitch (`self.LaunchWorldRotation`)) (* _rotationfloat 90.0)) (.yaw (`self.LaunchWorldRotation`))) false false))
        (:`Finished`
          (`self.ReturnRocket`)
          (`ResearchSystem.AuthorityGrantResearchPoints` 15))))
    (:`then_1`
      (goto _label_2))))

(event `self.ReceiveBeginPlay`
  (`parent.ReceiveBeginPlay`)
  (if (> (`self.LaunchAnimTimestamp`) 0.0)
    (goto _label)))

(fn `GetBodySlotLegacy`
  (returns (ReturnValue :type "ChildSlotComponent Object Reference"))
  (return (`self.RocketBodySlot`)))

(fn `UserConstructionScript`)