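; Small cargo rocket for the Space Storage mod that flies an ascent after launch, then delivers resources to the station and destroys itself.
; A timeline drives the mesh up and forward from the launch transform while pitching it over.
; The playback position is recorded in LaunchAnimTimestamp each update, so BeginPlay resumes an unfinished ascent from that point when the value is above zero.
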(event `self.OnLaunch`
  (bind _launchworldlocation (`self.LaunchWorldLocation`))
  (`parent.OnLaunch`)
  (set `self.LaunchAnimTimestamp` 0.0)
  (`|ExecutionSequence` :!label _label
    (:`then_0`
      (bind (_direction _rotationfloat _positionvertical _positionhorizontal) (`Timeline|Ascend Timeline` :`NewTime` (`self.LaunchAnimTimestamp`) :!via `SetNewTime` :!label _label_2)
        (:`Update`
          (set `self.LaunchAnimTimestamp` (`TimelineComponent.GetPlaybackPosition` (`self.Ascend Timeline`)))
          (`SceneComponent.K2_SetWorldLocationAndRotation` (`self.StaticMeshComponent`) (+ (`SceneComponent.K2_GetComponentLocation` (`self.LaunchWorldLocation`)) (* (`SceneComponent.GetUpVector` _launchworldlocation) (* _positionvertical 1900.0)) (* (`SceneComponent.GetForwardVector` _launchworldlocation) (* _positionhorizontal 15000.0))) (`KismetMathLibrary.MakeRotator` (.roll (`self.LaunchWorldRotation`)) (+ (.pitch (`self.LaunchWorldRotation`)) (* _rotationfloat -92.0)) (.yaw (`self.LaunchWorldRotation`))) false false))
        (:`Finished`
          (`self.OnDeliverResourcesToStation`)
          (`self.DestroyRocket`))))
    (:`then_1`
      (goto _label_2))))

(event `self.ReceiveBeginPlay`
  (`parent.ReceiveBeginPlay`)
  (if (> (`self.LaunchAnimTimestamp`) 0.0)
    (goto _label)))

(fn `UserConstructionScript`
  (`parent.UserConstructionScript`))