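; Large cargo rocket Blueprint for the Space Storage mod, animating a round trip that delivers resources to a station.
; Ascend and descend timelines drive mesh position and pitch from the launch transform, with delivery and a short timer between them.
; BeginPlay resumes an interrupted flight using the stored timestamp and Returning flag.
; In hydrazine mode, the slotted medium thruster is toggled by calling its use-input event, based on fuel level and descent progress.
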(event `self.OnLaunch`
  (bind _launchworldlocation (`self.LaunchWorldLocation`))
  (bind _staticmeshcomponent (`self.StaticMeshComponent`))
  (`parent.OnLaunch`)
  (set `self.SC_UpVector` (`SceneComponent.GetUpVector` _staticmeshcomponent))
  (set `self.SC_FwVector` (`KismetMathLibrary.NegateVector` (`SceneComponent.GetForwardVector` _staticmeshcomponent)))
  (if (`self.HydrazineFuelsMode`)
    (bind _physical_item (`/Game/Mods/Yzch/SpaceStorage/MoreSlotFunctions.GetSlotItem` (`self.ThrusterSlot`)))
    (bind _asthruster_medium (cast `/Game/Components_Medium/Thruster_Medium` _physical_item)
      (:`then`
        (set `self.HydrazineThruster` _asthruster_medium))
      (:`CastFailed`
        _)))
  (set `self.HydrazineThrusterActive` true)
  (set `self.LaunchAnimTimestamp` 0.0)
  (`|ExecutionSequence` :!label _label
    (:`then_0`
      (bind (_direction _rotationfloat _positionvertical _positionhorizontal) (`Timeline|Ascend Timeline` :`NewTime` (`self.LaunchAnimTimestamp`) :!via `SetNewTime` :!label _label_2)
        (:`Update`
          (set `self.LaunchAnimTimestamp` (`TimelineComponent.GetPlaybackPosition` (`self.Ascend Timeline`)))
          (`|ExecutionSequence`
            (:`then_0`
              (if (`self.HydrazineFuelsMode`)
                (bind _fuel (`/Game/Components_Medium/Thruster_Medium.GetAvailableFuel` (`self.HydrazineThruster`)))
                (if (and (< _fuel 1.1) (`self.HydrazineThrusterActive`))
                  (`/Game/Components_Medium/Thruster_Medium.InpActEvt_Use_K2Node_InputActionEvent_0` (`self.HydrazineThruster`))
                  (set `self.HydrazineThrusterActive` false))))
            (:`then_1`
              (`SceneComponent.K2_SetWorldLocationAndRotation` (`self.StaticMeshComponent`) (+ (`SceneComponent.K2_GetComponentLocation` (`self.LaunchWorldLocation`)) (* (`SceneComponent.GetUpVector` _launchworldlocation) (* _positionvertical 1900.0)) (* (`SceneComponent.GetForwardVector` _launchworldlocation) (* _positionhorizontal 15000.0))) (`KismetMathLibrary.MakeRotator` (.roll (`self.LaunchWorldRotation`)) (+ (.pitch (`self.LaunchWorldRotation`)) (* _rotationfloat -92.0)) (.yaw (`self.LaunchWorldRotation`))) false false))))
        (:`Finished`
          (`self.OnDeliverResourcesToStation`)
          (`KismetSystemLibrary.K2_SetTimerDelegate` (delegate `DescendEvent`) 3.0 false 3.0)
          (set `self.Returning` true))))
    (:`then_1`
      (goto _label_2))))

(event `self.ReceiveBeginPlay`
  (bind _launchworldlocation (`self.LaunchWorldLocation`))
  (bind _hydrazinefuelsmode (`self.HydrazineFuelsMode`))
  (bind _returnvalue (`TimelineComponent.GetPlaybackPosition` (`self.Descend Timeline`)))
  (`parent.ReceiveBeginPlay`)
  (if (`self.Returning`)
    (if (> (`self.LaunchAnimTimestamp`) 0.0)
      (`|ExecutionSequence` :!label _label_3
        (:`then_0`
          (bind (_direction _rotationfloat _positionvertical _positionhorizontal) (`Timeline|Descend Timeline` :`NewTime` (`self.LaunchAnimTimestamp`) :!via `SetNewTime` :!label _label_4)
            (:`Update`
              (set `self.LaunchAnimTimestamp` _returnvalue)
              (`|ExecutionSequence`
                (:`then_0`
                  (`SceneComponent.K2_SetWorldLocationAndRotation` (`self.StaticMeshComponent`) (+ (`SceneComponent.K2_GetComponentLocation` (`self.LaunchWorldLocation`)) (* (`SceneComponent.GetUpVector` _launchworldlocation) (* _positionvertical 1900.0)) (* (`SceneComponent.GetForwardVector` _launchworldlocation) (* _positionhorizontal -15000.0))) (`KismetMathLibrary.MakeRotator` (.roll (`self.LaunchWorldRotation`)) (+ (.pitch (`self.LaunchWorldRotation`)) (* _rotationfloat 92.0)) (.yaw (`self.LaunchWorldRotation`))) false false))
                (:`then_1`
                  (if (and (>= _returnvalue 13.0) _hydrazinefuelsmode)
                    (if (not (`self.HydrazineThrusterActive`))
                      (`/Game/Components_Medium/Thruster_Medium.InpActEvt_Use_K2Node_InputActionEvent_0` (`self.HydrazineThruster`))
                      (set `self.HydrazineThrusterActive` true))))))
            (:`Finished`
              (`|ExecutionSequence`
                (:`then_0`
                  (if _hydrazinefuelsmode
                    (`/Game/Components_Medium/Thruster_Medium.InpActEvt_Use_K2Node_InputActionEvent_0` (`self.HydrazineThruster`))))
                (:`then_1`
                  (`self.ReturnRocket`))))))
        (:`then_1`
          (goto _label_4))))
    (elif (> (`self.LaunchAnimTimestamp`) 0.0)
      (goto _label))))

(event `DescendEvent`
  (set `self.LaunchAnimTimestamp` 0.0)
  (goto _label_3))

(fn `UserConstructionScript`
  (`parent.UserConstructionScript`))