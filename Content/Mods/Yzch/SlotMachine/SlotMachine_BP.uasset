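; Slot machine that consumes the item in its resource slot on use and pays out copies of it when fruits match.
; Outside creative mode, non-resource items are ejected instead of played.
; Tick eases the lever and spins three reels at random speeds; a timer stops them sequentially, snapping each to one of six fruit positions.
; GetRewards counts matching pairs, then a looping timer launches the prize items and fires bonus rockets before re-enabling the machine.
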(event `SpawnRewardItem`
  ;[1 0 0.8568] Checking for rewards and counting
  (if (> (stale _output_get) 0)
    (bind _output_get (set `self.RewardsCount` (- (stale _output_get) 1)))
    ;[0.2318 1 0] Spawn main reward item
    (bind _returnvalue (`|SpawnActorFromClass` (`self.GamblingItem`) (`SceneComponent.K2_GetComponentToWorld` (`self.T1Resource`)) "AlwaysSpawn" "OverrideRootScale" null null))
    (`ItemComponent.SetItem` (`PhysicalItem.ItemComponent` _returnvalue) (`self.GamblingItemType`) (`ItemStatics.AmountFromRecipe` 1.0) false)
    (`KismetSystemLibrary.Delay` 0.05)
    (`self.LaunchItemIntoAir` _returnvalue)
    (elif (> (stale _output_get_2) 0)
      (bind _output_get_2 (set `self.RewardFireworks` (- (stale _output_get_2) 1)))
      ;[1 0.2021 0] Spawn firework item
      (bind _returnvalue_2 (`|SpawnActorFromClass` "/Game/Components_Medium/Firework_Rocket.Firework_Rocket_C" (`SceneComponent.K2_GetComponentToWorld` (`self.T1Resource`)) "AlwaysSpawn" "OverrideRootScale" null null))
      (`ItemComponent.SetItem` (`PhysicalItem.ItemComponent` _returnvalue_2) "/Game/Items/ItemTypes/Fireworks.Fireworks_C" (`ItemStatics.AmountFromRecipe` 1.0) false)
      (`KismetSystemLibrary.Delay` 0.05)
      (`/Game/Components_Medium/Firework_Rocket.InpActEvt_Use_K2Node_InputActionEvent_0` _returnvalue_2)
      (else
        ;[0 0.2004 1] Clear machine for next spin
        (`KismetSystemLibrary.K2_ClearAndInvalidateTimerHandle` (stale `StopMachine` _returnvalue) :!label _label)
        (`KismetSystemLibrary.Delay` 1.0)
        (set `self.Working` false)
        (set `ClickableComponent.Unclickable` false (`self.ClickableComponent`))))))

(event `self.ReceiveBeginPlay`
  (bind _staticmeshcomponent (`self.StaticMeshComponent`))
  ;[1 0.02273 0] Collision when slotted
  (`PrimitiveComponent.SetCollisionEnabled` _staticmeshcomponent "QueryAndPhysics" :!label _label_2)
  (`PrimitiveComponent.SetCollisionResponseToChannel` _staticmeshcomponent "ECC_Pawn" "ECR_Block"))

(event `StopMachine`
  (`KismetSystemLibrary.Delay` 0.5)
  (set `self.Spinning1` 0.0)
  (`AstroStatics.PlaySound` "/Game/Mods/Yzch/SlotMachine/Sounds/sfx_slotDing.sfx_slotDing")
  (`KismetSystemLibrary.Delay` 0.5)
  (set `self.Spinning2` 0.0)
  (`AstroStatics.PlaySound` "/Game/Mods/Yzch/SlotMachine/Sounds/sfx_slotDing.sfx_slotDing")
  (`KismetSystemLibrary.Delay` 0.5)
  (set `self.Spinning3` 0.0)
  (`AstroStatics.PlaySound` "/Game/Mods/Yzch/SlotMachine/Sounds/sfx_slotDing.sfx_slotDing")
  (`KismetSystemLibrary.Delay` 1.0)
  (bind (_reward _rewardfireworks) (`self.GetRewards`))
  (set `self.RewardFireworks` _rewardfireworks)
  (bind _output_get (set `self.RewardsCount` _reward))
  (if (== _output_get 0)
    (goto _label)
    (else
      (`AstroStatics.PlaySound` "/Game/Mods/Yzch/SlotMachine/Sounds/sfx_slotCoins.sfx_slotCoins")
      (bind _returnvalue (`KismetSystemLibrary.K2_SetTimerDelegate` (delegate `SpawnRewardItem`) 0.5 true)))))

(event `self.PickedUpFromWorld`
  ;[1 0.02273 0] Collision when slotted
  (goto _label_2))

(event `self.StartInWorld`
  ;[1 0.02273 0] Collision when slotted
  (goto _label_2))

(event `self.PlacedInSlot`
  (params (Slot :type "SlotReference Structure") (FromTool :type Boolean) (SlottedDuringInitialization :type Boolean))
  ;[1 0.02273 0] Collision when slotted
  (goto _label_2))

(event `InputAction|Use`
  (params (Key :type "Key Structure"))
  (bind _slotscomponent (`self.SlotsComponent`))
  (bind _returnvalue (`SlotsComponent.MakeReference` _slotscomponent "T1Resource"))
  (bind _returnvalue_2 (`SlotsComponent.GetSlotItem` _slotscomponent _returnvalue 0))
  (:`Pressed`
    (if (`self.Working`)
      _
      (elif (`AstroGameState.IsCreativeModeActive` (`AstroStatics.GetGameState`))
        (set `self.GamblingItem` (stale _asphysical_resource) :!label _label_3)
        (set `self.GamblingItemType` (`ItemComponent.ItemType` (`PhysicalItem.ItemComponent` _returnvalue_2)))
        (`SlotsComponent.DestroySlotItem` (`self.SlotsComponent`) _returnvalue)
        (set `self.Working` true)
        (set `self.LeverTargetRotation` -80.0)
        (`AstroStatics.PlaySound` "/Game/Mods/Yzch/SlotMachine/Sounds/sfx_slotUse.sfx_slotUse")
        (set `ClickableComponent.Unclickable` true (`self.ClickableComponent`))
        (`KismetSystemLibrary.Delay` 0.1)
        (`AstroStatics.PlaySound` "/Game/Mods/Yzch/SlotMachine/Sounds/sfx_slotSpinning.sfx_slotSpinning")
        (`KismetSystemLibrary.Delay` 0.5)
        (bind _speed (`self.RandomSpinSpeed`))
        (set `self.Spinning1` _speed)
        (`KismetSystemLibrary.Delay` 0.5)
        (bind _speed_2 (`self.RandomSpinSpeed`))
        (set `self.Spinning2` _speed_2)
        (`KismetSystemLibrary.Delay` 0.5)
        (bind _speed_3 (`self.RandomSpinSpeed`))
        (set `self.Spinning3` _speed_3)
        (set `self.LeverTargetRotation` 0.0)
        (`KismetSystemLibrary.K2_SetTimerDelegate` (delegate `StopMachine`) 4.0)
        (else
          (bind _asphysical_resource (castclass `PhysicalResource` (`GameplayStatics.GetObjectClass` _returnvalue_2))
            (:`then`
              (goto _label_3))
            (:`CastFailed`
              (`SlotsComponent.ReleaseItem` _returnvalue _returnvalue_2)
              (`KismetSystemLibrary.Delay` 0.5)
              (`self.LaunchItemIntoAir` _returnvalue_2))))))))

(event `self.ReceiveTick`
  (params (DeltaSeconds :type "Float (single-precision)"))
  (bind _returnvalue (`KismetMathLibrary.MakeRotator` 0.0 (* DeltaSeconds -1.0)))
  (if (`self.Working`)
    (`|ExecutionSequence`
      (:`then_0`
        (if (>= (`self.Spinning3`) 0.1)
          (`self.RotateSpin` (`self.Spin3`) (`self.SpinRot3`) (* _returnvalue (`self.Spinning3`)))
          (else
            (`self.SpinRotateToClosestFruit` (`self.Spin3`) (`self.SpinRot3`)))))
      (:`then_1`
        (if (>= (`self.Spinning2`) 0.1)
          (`self.RotateSpin` (`self.Spin2`) (`self.SpinRot2`) (* _returnvalue (`self.Spinning2`)))
          (else
            (`self.SpinRotateToClosestFruit` (`self.Spin2`) (`self.SpinRot2`)))))
      (:`then_2`
        (if (>= (`self.Spinning1`) 0.1)
          (`self.RotateSpin` (`self.Spin1`) (`self.SpinRot1`) (* _returnvalue (`self.Spinning1`)))
          (else
            (`self.SpinRotateToClosestFruit` (`self.Spin1`) (`self.SpinRot1`)))))
      (:`then_3`
        (`self.RotateSpin` (`self.Lever`) (`self.LeverRot`) (`KismetMathLibrary.MakeRotator` 0.0 (* (* DeltaSeconds 10.0) (- (`self.LeverTargetRotation`) (.pitch (`self.LeverRot`))))))))))

(fn `GetBodySlotLegacy`
  (returns (ReturnValue :type "ChildSlotComponent Object Reference"))
  (return (`self.BodySlot`)))

(fn `GetRewards`
  (returns (Reward :type Integer) (RewardFireworks :type Integer))
  (locals (matches :type Integer) (Fruit1 :type Integer) (Fruit2 :type Integer) (Fruit3 :type Integer))
  (bind _matches (`local.matches`))
  (`|ExecutionSequence`
    (:`then_0`
      ;[1 0 0] Get fruit ID
      (bind _fruitid (`self.SpinGetClosestFruitId` (`self.Spin1`) (`self.SpinRot1`)))
      (set `local.Fruit1` _fruitid))
    (:`then_1`
      (bind _fruitid_2 (`self.SpinGetClosestFruitId` (`self.Spin2`) (`self.SpinRot2`)))
      (set `local.Fruit2` _fruitid_2))
    (:`then_2`
      (bind _fruitid_3 (`self.SpinGetClosestFruitId` (`self.Spin3`) (`self.SpinRot3`)))
      (set `local.Fruit3` _fruitid_3))
    (:`then_3`
      ;[0 1 0.1106] Calculate matches
      (`|ExecutionSequence`
        (:`then_0`
          (if (== (`local.Fruit1`) (`local.Fruit2`))
            (bind _result (`/Engine/EditorBlueprintResources/StandardMacros.IncrementInt` (`local.matches`))
              (:`  `
                (set `local.matches` _result)))))
        (:`then_1`
          (if (== (`local.Fruit1`) (`local.Fruit3`))
            (bind _result_2 (`/Engine/EditorBlueprintResources/StandardMacros.IncrementInt` (`local.matches`))
              (:`  `
                (set `local.matches` _result_2)))))
        (:`then_2`
          (if (== (`local.Fruit2`) (`local.Fruit3`))
            (bind _result_3 (`/Engine/EditorBlueprintResources/StandardMacros.IncrementInt` (`local.matches`))
              (:`  `
                (set `local.matches` _result_3)))))))
    (:`then_4`
      ;[1 0.9939 0] Make rewards
      (if (== _matches 0)
        (return 0 0)
        (elif (== _matches 1)
          (return (`KismetMathLibrary.RandomIntegerInRange` 1 4) 1)
          (elif (== _matches 3)
            (return (`KismetMathLibrary.RandomIntegerInRange` 5 10) 5)))))))

(fn `LaunchItemIntoAir`
  (params (PhysicalItem :type "PhysicalItem Object Reference"))
  (`PrimitiveComponent.AddImpulse` (`PhysicalItem.StaticMeshComponent` PhysicalItem) (* (`self.GetActorUpVector` PhysicalItem) 1900.0) "None" true)
  (`AstroStatics.PlaySound` "/Game/Mods/Yzch/SlotMachine/Sounds/sfx_slotItemPop.sfx_slotItemPop"))

(fn `RandomSpinSpeed`
  (returns (Speed :type "Float (double-precision)"))
  (return (`KismetMathLibrary.RandomFloatInRange` 350.0 800.0)))

(fn `RotateSpin`
  (params (Spin :type "StaticMeshComponent Object Reference") (SpinRotator :type "Rotator Structure (by ref)") (Degrees :type "Rotator Structure"))
  (bind _returnvalue (`KismetMathLibrary.MakeRotator` 0.0 (mod (+ (.pitch SpinRotator) (.pitch Degrees)) -360.0)))
  (`SceneComponent.K2_SetRelativeRotation` Spin _returnvalue false false)
  (`|VariableSetRef` SpinRotator _returnvalue))

(fn `SpinGetClosestFruitId`
  (params (Spin :type "StaticMeshComponent Object Reference") (SpinRotator :type "Rotator Structure (by ref)"))
  (returns (fruitId :type Integer))
  (locals (Counting :type Integer) (PitchY :type "Float (double-precision)"))
  (bind _pitch (.pitch SpinRotator))
  (if (>= _pitch -30.0)
    (set `local.Counting` 0)
    (elif (>= _pitch -90.0)
      (set `local.Counting` 1)
      (elif (>= _pitch -150.0)
        (set `local.Counting` 2)
        (elif (>= _pitch -210.0)
          (set `local.Counting` 3)
          (elif (>= _pitch -270.0)
            (set `local.Counting` 4)
            (elif (>= _pitch -330.0)
              (set `local.Counting` 5)
              (else
                (set `local.Counting` 0))))))))
  (return (`local.Counting`)))

(fn `SpinRotateToClosestFruit`
  (params (Spin :type "StaticMeshComponent Object Reference") (SpinRotator :type "Rotator Structure (by ref)"))
  (bind _fruitid (`self.SpinGetClosestFruitId` Spin SpinRotator))
  (bind _returnvalue (* (struct :`Pitch` -60.0) _fruitid))
  (`|VariableSetRef` SpinRotator _returnvalue)
  (`SceneComponent.K2_SetRelativeRotation` Spin _returnvalue false false))

(fn `UserConstructionScript`)