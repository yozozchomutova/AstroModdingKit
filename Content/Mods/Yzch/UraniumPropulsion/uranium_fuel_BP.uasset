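; Uranium fuel canister Blueprint from the UraniumPropulsion mod, extending a parent item's construction script without adding live logic to it.
; TestFunc forces the ItemComponent's capacity, amount and fullness, refreshes the canister visuals and makes the item and its current slot clickable.
; No call to TestFunc appears here; a looping timer and a green tint for the resource bar and indicator ring are left disconnected.
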(fn `TestFunc`
  (bind _itemcomponent (`self.ItemComponent`))
  (set `ItemComponent.Capacity` 3.0 _itemcomponent)
  (`ItemComponent.SetAmount` _itemcomponent 3 false)
  (`ItemComponent.SetAmountUsingFullness` _itemcomponent 3.0 false)
  (`self.UpdateCanisterVisuals`)
  (`SlotsComponent.SetSlotClickable` (`self.CurrentSlot`) true)
  (set `ClickableComponent.Unclickable` false (`self.ClickableComponent`)))

(fn `UserConstructionScript`
  (`parent.UserConstructionScript`))