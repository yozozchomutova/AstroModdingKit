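; Nuclear thruster Blueprint from the UraniumPropulsion mod, a child thruster that pushes with a large fixed force and burns fuel.
; UpdateThrusterMotion applies force along the actor's up vector to StaticMeshComponent at the ThrustPoint location, shifted by the offset from its owner, then calls TakeFuel.
; The TakeFuel override multiplies the requested rate fivefold before passing it to the parent implementation.
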(event `self.UpdateThrusterMotion`
  (bind _returnvalue (`self.GetOffsetFromOwner`))
  (`AstroPlayStatics.AddComponentForceAtLocation` (`self.StaticMeshComponent`) (* (`self.GetActorUpVector`) 20000000.0) (+ (`SceneComponent.K2_GetComponentLocation` (`self.Thrust Point`)) _returnvalue))
  (`self.Take Fuel` 0.1))

(fn `Take Fuel`
  (params (Rate :type "Float (double-precision)"))
  (returns (Taken :type "Float (double-precision)"))
  (bind _taken (`parent.Take Fuel` (* Rate 5.0)))
  (return _taken))

(fn `UserConstructionScript`
  (`parent.UserConstructionScript`))