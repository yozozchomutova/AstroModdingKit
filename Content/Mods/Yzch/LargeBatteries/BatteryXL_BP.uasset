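; BatteryXL_BP is an extra-large battery from the LargeBatteries mod that shows its charge level through a moving indicator mesh.
; BeginPlay assigns the collision and indicator mesh references before calling the parent logic.
; On start and on each power level update, it raises or lowers the poseable mesh's "Top" bone by charge-to-capacity ratio.
; The indicator material's Fullness stays at full, so bone height alone conveys the level.
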(event `self.ReceiveBeginPlay`
  (bind _powercomponent (`self.PowerComponent`))
  (set `self.CollisionMeshComponent` (`self.StaticMeshComponent`))
  (set `self.IndicatorMesh` (`self.PoseableMesh`))
  (set `self.IndicatorMeshIndex` 1)
  (`parent.ReceiveBeginPlay`)
  (`PoseableMeshComponent.SetBoneLocationByName` (`self.PoseableMesh`) "Top" (`KismetMathLibrary.MakeVector` 0.0 0.0 (+ (* (/ (`PowerComponent.CurrentCharge` _powercomponent) (`PowerComponent.StorageCapacity` _powercomponent)) 590.0) 180.0)) "ComponentSpace" :!label _label)
  (`MaterialInstanceDynamic.SetScalarParameterValue` (`self.IndicatorMaterial`) "Fullness" 1.0))

(event `self.OnPowerLevelUpdate`
  (params (NewPower :type "Float (single-precision)") (Fullness :type "Float (single-precision)"))
  (goto _label))

(fn `UserConstructionScript`
  (`parent.UserConstructionScript`))