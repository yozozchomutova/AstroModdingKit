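; Small liquid tank item in the Liquids mod, a child Blueprint that sets a fixed fluid capacity on BeginPlay.
; It binds a visual update event to the parent's UV callback and triggers it once at start.
; The update shows the fill level by sliding a FluidMesh bone vertically in component space, lerped by current over max fluid, then refreshes the description.
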(event `self.ReceiveBeginPlay`
  (set `self.FluidMax` 16.0)
  (`parent.ReceiveBeginPlay`)
  (add `self.UV` (delegate `Update Visuals Event`))
  (`self.UV`))

(event `Update Visuals Event`
  (`PoseableMeshComponent.SetBoneLocationByName` (`self.FluidMesh`) "Root_001" (`KismetMathLibrary.MakeVector` 0.0 0.0 (`KismetMathLibrary.Lerp` -22.1 71.379997 (/ (`self.FluidCurrent`) (`self.FluidMax`)))) "ComponentSpace")
  (`self.UpdateDescription`))

(fn `UpdateVisualss`)

(fn `UserConstructionScript`
  (`parent.UserConstructionScript`))