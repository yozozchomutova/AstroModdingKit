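; Organic water extractor item that turns organic resources into dirty water for a liquid canister.
; Slot delegates track the organic input and output tank, with an indicator requesting organic material.
; Tick enables power while both are present and the canister can accept dirty water, then drains the organic and fills the canister proportionally to power load.
; A depleted organic item is destroyed, restoring the indicator and disabling power.
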(event `self.ReceiveBeginPlay`
  (bind _returnvalue (`SlotsComponent.GetSlotDelegates` (`ChildSlotComponent.MakeReference` (`self.OutputSlot`))))
  (bind _returnvalue_2 (`SlotsComponent.GetSlotDelegates` (`ChildSlotComponent.MakeReference` (`self.OrganicSlot`))))
  (`|ExecutionSequence`
    (:`then_0`
      (add `SlotDelegates.OnSetItem` _returnvalue_2 (delegate `Placed In Slot`))
      (add `SlotDelegates.OnReleaseItem` _returnvalue_2 (delegate `Released From Slot`))
      (`self.RefreshSlotIndicator` :!label _label)
      (`PowerComponent.SetEnabled` (`self.PowerComponent`) false))
    (:`then_1`
      (add `SlotDelegates.OnSetItem` _returnvalue (delegate `Placed in Slot Output`))
      (add `SlotDelegates.OnReleaseItem` _returnvalue (delegate `Released from Slot Output`)))))

(event `Placed In Slot`
  (params (Item :type "PhysicalItem Object Reference"))
  (set `self.OrganicResource` Item))

(event `Released From Slot`
  (params (Item :type "PhysicalItem Object Reference"))
  (set `self.OrganicResource` null)
  (goto _label))

(event `Placed in Slot Output`
  (params (Item :type "PhysicalItem Object Reference"))
  (bind _asliquid_tank_parent (cast `/Game/Mods/Yzch/Liquids/Items/LiquidTank_Parent` Item))
  (set `self.LiquidCanister` _asliquid_tank_parent))

(event `Released from Slot Output`
  (params (Item :type "PhysicalItem Object Reference"))
  (set `self.LiquidCanister` null)
  (`PowerComponent.SetEnabled` (`self.PowerComponent`) false))

(event `self.ReceiveTick`
  (params (DeltaSeconds :type "Float (single-precision)"))
  (bind _liquidcanister (`self.LiquidCanister`))
  (bind _itemcomponent (`PhysicalItem.ItemComponent` (`self.OrganicResource`)))
  (bind _returnvalue (* DeltaSeconds (`KismetMathLibrary.Abs` (`PowerComponent.NetActualLoad` (`self.PowerComponent`))) 0.01))
  (bind _returnvalue_2 (`KismetMathLibrary.FMax` (- (`ItemComponent.GetFullness` _itemcomponent) _returnvalue)))
  (if (and (!= (`self.LiquidCanister`) null) (!= (`self.OrganicResource`) null))
    (bind _can (`/Game/Mods/Yzch/Liquids/Items/LiquidTank_Parent.CanAddFluid` _liquidcanister "dirty_water"))
    (bind _is_full (`/Game/Mods/Yzch/Liquids/Items/LiquidTank_Parent.IsFull` _liquidcanister))
    (bind _returnvalue_3 (and _can (not _is_full)))
    (`PowerComponent.SetEnabled` (`self.PowerComponent`) _returnvalue_3)
    (if _returnvalue_3
      (`ItemComponent.SetAmountUsingFullness` _itemcomponent _returnvalue_2 false)
      (`/Game/Mods/Yzch/Liquids/Items/LiquidTank_Parent.AddFluid` (`self.LiquidCanister`) "dirty_water" (* _returnvalue 8.0))
      (if (<= _returnvalue_2 0.0)
        (`SlotsComponent.DestroySlotItem` (`self.SlotsComponent`) (`ChildSlotComponent.MakeReference` (`self.OrganicSlot`)))
        (set `self.OrganicResource` null)
        (`self.RefreshSlotIndicator`)
        (`PowerComponent.SetEnabled` (`self.PowerComponent`) false)))))

(fn `GetBodySlotLegacy`
  (returns (ReturnValue :type "ChildSlotComponent Object Reference"))
  (return (`self.BodySlot`)))

(fn `RefreshSlotIndicator`
  (`SlotsComponent.SlotAttemptToPushIndicatorIntoSpecificSubslot` (`ChildSlotComponent.MakeReference` (`self.OrganicSlot`)) 0 (make `SlotIndicatorDefinition` "/Game/Items/ItemTypes/Minables/Organic.Organic_C")))

(fn `UserConstructionScript`)