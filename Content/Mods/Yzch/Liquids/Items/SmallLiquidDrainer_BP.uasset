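; Blueprint for a small liquid drainer item that slowly empties a liquid tank placed in its tank slot.
; On BeginPlay a looping timer checks the slot every tenth of a second.
; When the slot holds an item that casts to LiquidTank_Parent, it removes a small fixed amount of fluid from it.
; It also exposes its body slot through the legacy getter.
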(event `self.ReceiveBeginPlay`
  (`KismetSystemLibrary.K2_SetTimerDelegate` (delegate `CheckTank`) 0.1 true))

(event `CheckTank`
  (bind _returnvalue (`ChildSlotComponent.MakeReference` (`self.TankSlot`)))
  (if (`SlotStatics.HasAnyItem` _returnvalue)
    (bind _asliquid_tank_parent (cast `/Game/Mods/Yzch/Liquids/Items/LiquidTank_Parent` (`SlotsComponent.GetSlotPrimaryItem` _returnvalue)))
    (`/Game/Mods/Yzch/Liquids/Items/LiquidTank_Parent.RemoveFluid` _asliquid_tank_parent 0.05)))

(event `self.ReceiveTick`
  (params (DeltaSeconds :type "Float (single-precision)")))

(fn `GetBodySlotLegacy`
  (returns (ReturnValue :type "ChildSlotComponent Object Reference"))
  (return (`self.BodySlot`)))

(fn `UserConstructionScript`)