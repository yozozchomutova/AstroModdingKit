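; Plantable pot item for the AstroVitals mod that grows fruit from seeds and yields it on harvest.
; Its input slot takes clay as soil, liquid tank fluid as water and seeds to choose the fruit.
; A looping timer randomly advances watered growth on certain planets; Use harvests, wearing down soil and plant, or clears an unripe plant.
; UpdateState refreshes staged plant meshes, fruit meshes borrowed from item class defaults, and tooltip status.
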(event `self.PickedUpFromWorld`
  (bind _staticmeshcomponent (`self.StaticMeshComponent`))
  ;[1 0.02273 0] Collision when slotted
  (`PrimitiveComponent.SetCollisionEnabled` _staticmeshcomponent "QueryAndPhysics" :!label _label)
  (`PrimitiveComponent.SetCollisionResponseToChannel` _staticmeshcomponent "ECC_Pawn" "ECR_Block"))

(event `self.StartInWorld`
  ;[1 0.02273 0] Collision when slotted
  (goto _label))

(event `self.PlacedInSlot`
  (params (Slot :type "SlotReference Structure") (FromTool :type Boolean) (SlottedDuringInitialization :type Boolean))
  ;[1 0.02273 0] Collision when slotted
  (goto _label))

(event `self.ReceiveBeginPlay`
  (`|ExecutionSequence`
    (:`then_0`
      (goto _label))
    (:`then_1`
      (add `SlotDelegates.OnSetItem` (`SlotsComponent.GetSlotDelegates` (`ChildSlotComponent.MakeReference` (`self.Input Slot`))) (delegate `On Input Item Placed`)))
    (:`then_2`
      (`self.UpdateState`))
    (:`then_3`
      (`KismetSystemLibrary.K2_SetTimerDelegate` (delegate `5 Sec Event`) 5.0 true 3.0))))

(event `On Input Item Placed`
  (params (Item :type "PhysicalItem Object Reference"))
  (if (== "/Game/Items/ItemTypes/Minables/Clay.Clay_C" (`ItemComponent.ItemType` (`PhysicalItem.ItemComponent` Item)))
    (`self.AddDirt` 4)
    (set `self.Watered` false)
    (`SlotsComponent.DestroySlotItem` (`ChildSlotComponent.MakeReference` (`self.Input Slot`)) :!label _label_2)
    (`self.UpdateState` :!label _label_3)
    (elif (not (`self.Watered`))
      (bind _asliquid_tank_parent (cast `/Game/Mods/Yzch/Liquids/Items/LiquidTank_Parent` Item)
        (:`then`
          (if (>= (`/Game/Mods/Yzch/Liquids/Items/LiquidTank_Parent.FluidCurrent` _asliquid_tank_parent) 1.0)
            (bind _success (`/Game/Mods/Yzch/Liquids/Items/LiquidTank_Parent.RemoveFluid` _asliquid_tank_parent 1.0))
            (set `self.Watered` _success)
            (goto _label_3)))
        (:`CastFailed`
          (if (> (`self.DirtDurability`) 0) :!label _label_4
            (bind _asfruit_seed_bp (cast `/Game/Mods/Yzch/AstroVitals/Items/FruitSeed_BP` Item))
            (set `self.FruitToSpawn` (`/Game/Mods/Yzch/AstroVitals/Items/FruitSeed_BP.Fruit` _asfruit_seed_bp))
            (set `self.GrowProgress` 0.0)
            (set `self.TreeDurability` 2)
            (goto _label_2))))
      (else
        (goto _label_4)))))

(event `5 Sec Event`
  (switch `EPlanetIdentifier` (`AstroPlanet.PlanetIdentifier` (`PlanetStatics.GetPlanet` self))
    (:`Terran`
      _)
    (:`Exotic`
      _)
    (:`ExoticMoon`
      _)
    (:`Arid`
      _))
  (if (and (!= null (`self.FruitToSpawn`)) (`self.Watered`))
    (if (not (>= (`self.GrowProgress`) 100.0))
      (bind _output_get (set `self.GrowProgress` (+ (stale _output_get) (`KismetMathLibrary.RandomFloatInRange` 0.694444 1.190476)))))
    (`self.UpdateState`)))

(event `InputAction|Use`
  (params (Key :type "Key Structure"))
  (bind _dirtdurability (`self.DirtDurability`))
  (bind _treedurability (`self.TreeDurability`))
  (:`Pressed`
    (if (>= (`self.GrowProgress`) 100.0)
      (for _ (range 3)
        (`SlotsComponent.SpawnItemTypeInSlot` (`ChildSlotComponent.MakeReference` (`self.Input Slot`)) (`self.FruitToSpawn`) true))
      (set `self.TreeDurability` (`KismetMathLibrary.Max` (- _treedurability 1)))
      (set `self.DirtDurability` (`KismetMathLibrary.Max` (- _dirtdurability 1)))
      (if (not (and (> _treedurability 0) (> _dirtdurability 0)))
        (set `self.FruitToSpawn` null :!label _label_5))
      (set `self.Watered` false)
      (set `self.GrowProgress` 0.0)
      (`self.UpdateState`)
      (elif (!= null (`self.FruitToSpawn`))
        (set `self.DirtDurability` (`KismetMathLibrary.Max` (- (`self.DirtDurability`) 1)))
        (set `self.TreeDurability` 0)
        (goto _label_5)))))

(fn `AddDirt`
  (params (Amount :type Integer))
  (bind _output_get (set `self.DirtDurability` (+ (stale _output_get) Amount)))
  (bind _output_get_2 (set `self.DirtDurability` (`KismetMathLibrary.Clamp` (stale _output_get_2) 0 (`self.DirtMax`)))))

(fn `GetBodySlotLegacy`
  (returns (ReturnValue :type "ChildSlotComponent Object Reference"))
  (return (`self.Body`)))

(fn `UpdateState`
  (locals (ItemDescription :type String))
  (bind _array (`|MakeArray` (`self.Food_1`) (`self.Food_2`) (`self.Food_3`)))
  (`|ExecutionSequence`
    (:`then_0`
      (`SceneComponent.SetVisibility` (`self.DirtMesh`) (> (`self.DirtDurability`) 0) false))
    (:`then_1`
      (if (> (`self.DirtDurability`) 0)
        (if (!= (`self.FruitToSpawn`) null)
          (if (`self.Watered`)
            (if (>= (`self.GrowProgress`) 100.0)
              (set `local.ItemDescription` "Ready to harvest!")
              (setmembers `TooltipWidgetDisplayData` :`StructRef` (`TooltipComponent.DefaultDisplayData` (`self.TooltipComponent`)) :`InteractionPrompts` (`|MakeArray` (make `InteractionPromptEntryData` "Use" "None" "None" 0.0 false "Harvest")))
              (else
                (set `local.ItemDescription` "Growing...")
                (setmembers `TooltipWidgetDisplayData` :`StructRef` (`TooltipComponent.DefaultDisplayData` (`self.TooltipComponent`)) :`InteractionPrompts` (`|MakeArray` (make `InteractionPromptEntryData` "Use" "None" "None" 0.0 false "Clear")))))
            (else
              (set `local.ItemDescription` "Needs a water!")
              (setmembers `TooltipWidgetDisplayData` :`StructRef` (`TooltipComponent.DefaultDisplayData` (`self.TooltipComponent`)) :`InteractionPrompts` (`|MakeArray`) :!label _label)))
          (else
            (set `local.ItemDescription` "Needs a seed!")
            (goto _label)))
        (else
          (set `local.ItemDescription` "Needs a clay!")
          (goto _label))))
    (:`then_2`
      (`self.UpdateTooltipDescription` (`local.ItemDescription`)))
    (:`then_3`
      (`SceneComponent.SetVisibility` (`self.Plant_1`) (!= null (`self.FruitToSpawn`)) false)
      (`SceneComponent.SetVisibility` (`self.Plant_2`) (>= (`self.GrowProgress`) 25.0) false)
      (`SceneComponent.SetVisibility` (`self.Plant_3`) (>= (`self.GrowProgress`) 50.0) false)
      (`SceneComponent.SetVisibility` (`self.Plant_4`) (>= (`self.GrowProgress`) 75.0) false)
      (if (< (`self.GrowProgress`) 100.0)
        (for _array_element _array
          (`StaticMeshComponent.SetStaticMesh` _array_element null :!label _label_2))
        (else
          (bind _asphysical_item (castclass `PhysicalItem` (defaults `/Game/Mods/Yzch/AstroVitals/Items/T1_pot_BP` (`self.FruitToSpawn`))))
          (for _array_element_2 _array
            (if (== (`self.FruitToSpawn`) "/Game/Items/ItemTypes/Minables/Organic.Organic_C")
              (goto _label_2)
              (else
                (`StaticMeshComponent.SetStaticMesh` _array_element_2 (`StaticMeshComponent.StaticMesh` (`PhysicalItem.StaticMeshComponent` (`ItemStatics.PhysicalItemDefault` _asphysical_item))))))))))))

(fn `UpdateTooltipDescription`
  (params (`Item Description` :type String))
  (setmembers `TooltipWidgetDisplayData` :`StructRef` (`TooltipComponent.DefaultDisplayData` (`self.TooltipComponent`)) :`Description` (`KismetTextLibrary.Conv_StringToText` (`KismetStringLibrary.Concat_StrStr` (`KismetStringLibrary.Concat_StrStr` "Fruit: " (`self.FruitToSpawnName`) " (" (`KismetStringLibrary.Conv_IntToString` (`KismetMathLibrary.Round` (`self.GrowProgress`))) "%)") "" " \nSoil: " (`KismetStringLibrary.Conv_IntToString` (`self.DirtDurability`)) "/" (`KismetStringLibrary.Conv_IntToString` (`self.DirtMax`)) " \nPlant durability: " (`KismetStringLibrary.Conv_IntToString` (`self.TreeDurability`)) " \nWatered: " (select `bool` (`self.Watered`) :`false` "No" :`true` "Yes") " \n \n" `Item Description`))))

(fn `UserConstructionScript`)