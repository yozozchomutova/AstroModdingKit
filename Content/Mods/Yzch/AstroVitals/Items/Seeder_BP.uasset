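; Seeder machine for the AstroVitals mod that turns an Organic item in its slot into a fruit seed.
; Four control panel buttons pick the seed type (cherry, banana, tomato or organic), switching power on and toggling the panel light.
; Tick spins the rotary and drains the Organic at a rate scaled by power load.
; Once empty, the item is replaced in-slot by a FruitSeed_BP of the chosen type and power shuts off.
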(event `Btn_1 Clicked`
  (`self.StartMakingSeed` "/Game/Mods/Yzch/AstroVitals/Items/Cherry_IT.Cherry_IT_C"))

(event `Btn_2 Clicked`
  (`self.StartMakingSeed` "/Game/Mods/Yzch/AstroVitals/Items/Banana_IT.Banana_IT_C"))

(event `Btn_3 Clicked`
  (`self.StartMakingSeed` "/Game/Mods/Yzch/AstroVitals/Items/Tomato_IT.Tomato_IT_C"))

(event `Btn_4 Clicked`
  (`self.StartMakingSeed` "/Game/Items/ItemTypes/Minables/Organic.Organic_C"))

(event `self.ReceiveBeginPlay`
  (bind _returnvalue (`SlotsComponent.GetSlotDelegates` (`ChildSlotComponent.MakeReference` (`self.OrganicSlot`))))
  (`|ExecutionSequence`
    (:`then_0`
      (bind _asseeder_panel (cast `/Game/Mods/Yzch/AstroVitals/Seeder_Panel` (`ChildActorComponent.ChildActor` (`self.SeederControlpanel`))))
      (bind _output_get (set `self.Seeder Control Panel` _asseeder_panel))
      (bind _seeder_panel_ui (`/Game/Mods/Yzch/AstroVitals/Seeder_Panel.Get Seeder Panel UI` _output_get))
      (add `Button.OnClicked` (`/Game/Mods/Yzch/AstroVitals/Seeder_Panel_UI.btn_1` _seeder_panel_ui) (delegate `Btn_1 Clicked`))
      (add `Button.OnClicked` (`/Game/Mods/Yzch/AstroVitals/Seeder_Panel_UI.btn_2` _seeder_panel_ui) (delegate `Btn_2 Clicked`))
      (add `Button.OnClicked` (`/Game/Mods/Yzch/AstroVitals/Seeder_Panel_UI.btn_3` _seeder_panel_ui) (delegate `Btn_3 Clicked`))
      (add `Button.OnClicked` (`/Game/Mods/Yzch/AstroVitals/Seeder_Panel_UI.btn_4` _seeder_panel_ui) (delegate `Btn_4 Clicked`)))
    (:`then_1`
      (add `SlotDelegates.OnSetItem` _returnvalue (delegate `Placed In Slot`))
      (add `SlotDelegates.OnReleaseItem` _returnvalue (delegate `Released From Slot`))
      (`self.RefreshIndicator`))
    (:`then_2`
      (if (== null (`self.OrganicItem`))
        (set `self.SelectedFruit` null)))))

(event `Placed In Slot`
  (params (Item :type "PhysicalItem Object Reference"))
  (set `self.OrganicItem` Item))

(event `Released From Slot`
  (params (Item :type "PhysicalItem Object Reference"))
  (`self.RefreshIndicator`))

(event `self.ReceiveTick`
  (params (DeltaSeconds :type "Float (single-precision)"))
  (bind _returnvalue (`ChildSlotComponent.MakeReference` (`self.OrganicSlot`)))
  (bind _itemcomponent (`PhysicalItem.ItemComponent` (`self.OrganicItem`)))
  (bind _returnvalue_2 (`KismetMathLibrary.Abs` (`PowerComponent.NetActualLoad` (`self.PowerComponent`))))
  (bind _returnvalue_3 (`KismetMathLibrary.FMax` (- (`ItemComponent.GetFullness` _itemcomponent) (* DeltaSeconds _returnvalue_2 0.02))))
  (if (not (== (`self.SelectedFruit`) null))
    (`SceneComponent.K2_AddLocalRotation` (`self.Rotary`) (`KismetMathLibrary.MakeRotator` 0.0 0.0 (* DeltaSeconds _returnvalue_2 40.0)) false false)
    (`ItemComponent.SetAmountUsingFullness` _itemcomponent _returnvalue_3 false)
    (if (<= _returnvalue_3 0.0)
      (`SlotsComponent.DestroySlotItem` (`self.SlotsComponent`) _returnvalue)
      (set `self.OrganicItem` null)
      (bind _returnvalue_4 (`SlotsComponent.SpawnActorInSlot` _returnvalue "/Game/Mods/Yzch/AstroVitals/Items/FruitSeed_BP.FruitSeed_BP_C"))
      (bind _asfruit_seed_bp (cast `/Game/Mods/Yzch/AstroVitals/Items/FruitSeed_BP` _returnvalue_4))
      (set `/Game/Mods/Yzch/AstroVitals/Items/FruitSeed_BP.Fruit` (`self.SelectedFruit`) _asfruit_seed_bp)
      (set `self.SelectedFruit` null)
      (set `self.OrganicItem` null)
      (`/Game/Mods/Yzch/AstroVitals/Seeder_Panel.SwitchLight` (`self.Seeder Control Panel`) true)
      (`PowerComponent.SetEnabled` (`self.PowerComponent`) false))))

(fn `GetBodySlotLegacy`
  (returns (ReturnValue :type "ChildSlotComponent Object Reference"))
  (return (`self.BodySlot`)))

(fn `RefreshIndicator`
  (`SlotsComponent.SlotAttemptToPushIndicatorIntoSpecificSubslot` (`ChildSlotComponent.MakeReference` (`self.OrganicSlot`)) 0 (make `SlotIndicatorDefinition` "/Game/Items/ItemTypes/Minables/Organic.Organic_C")))

(fn `StartMakingSeed`
  (params (`Seed Type` :type "ItemType Class Reference"))
  (if (and (== (`ItemComponent.ItemType` (`PhysicalItem.ItemComponent` (`self.OrganicItem`))) "/Game/Items/ItemTypes/Minables/Organic.Organic_C") (== (`self.SelectedFruit`) null))
    (set `self.SelectedFruit` `Seed Type`)
    (`/Game/Mods/Yzch/AstroVitals/Seeder_Panel.SwitchLight` (`self.Seeder Control Panel`) false)
    (`PowerComponent.SetEnabled` (`self.PowerComponent`) true)))

(fn `UserConstructionScript`)