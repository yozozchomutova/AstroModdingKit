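; FruitSeed_BP is a seed item in the AstroVitals mod that carries a Fruit value identifying what it grows.
; On BeginPlay it reassigns Fruit to itself, which appears intended to fire the OnRep_Fruit notify.
; That notify rebuilds the tooltip description from the fruit's default control symbol name, labelling it as a growable type.
; A legacy getter exposes the item's body slot.
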(event `self.ReceiveBeginPlay`
  (set `self.Fruit` (`self.Fruit`)))

(fn `GetBodySlotLegacy`
  (returns (ReturnValue :type "ChildSlotComponent Object Reference"))
  (return (`self.Body Slot`)))

(fn `OnRep_Fruit`
  (setmembers `TooltipWidgetDisplayData` :`StructRef` (`TooltipComponent.DefaultDisplayData` (`self.TooltipComponent`)) :`Description` (`KismetTextLibrary.Conv_StringToText` (`KismetStringLibrary.Concat_StrStr` "Type: " (`KismetTextLibrary.Conv_TextToString` (`ControlSymbol.Name` (`AstroPlayStatics.GetControlSymbolDefault` (`self.Fruit`)))) " \nGrowable"))))

(fn `UserConstructionScript`)