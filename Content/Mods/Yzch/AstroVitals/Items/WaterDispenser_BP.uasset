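; Water dispenser item for the AstroVitals mod that stores fluid and lets the player drink from it, reporting the amount drunk to HungerManager.
; A looping timer tops up the tank in the bottle slot from the dispenser and drains the input slot's tank into it, always adding as "dirty_water".
; A bound update event moves a FluidMesh bone to show the fill level and refreshes the description.
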(event `CheckTank`
  (bind _returnvalue (`ChildSlotComponent.MakeReference` (`self.BottleSlot`)))
  (bind _returnvalue_2 (`ChildSlotComponent.MakeReference` (`self.InputSlot`)))
  (`|ExecutionSequence`
    (:`then_0`
      (if (`SlotStatics.HasAnyItem` _returnvalue)
        (bind _asliquid_tank_parent (cast `/Game/Mods/Yzch/Liquids/Items/LiquidTank_Parent` (`SlotsComponent.GetSlotPrimaryItem` _returnvalue)))
        (bind _value (`self.HowMuchCanBeInserted` _asliquid_tank_parent))
        (bind (_success _amountactuallyremoved) (`self.RemoveFluid` (`KismetMathLibrary.FMin` _value 0.1)))
        (`self.AddFluid` _asliquid_tank_parent "dirty_water" _amountactuallyremoved)))
    (:`then_1`
      (if (`SlotStatics.HasAnyItem` _returnvalue_2)
        (bind _asliquid_tank_parent_2 (cast `/Game/Mods/Yzch/Liquids/Items/LiquidTank_Parent` (`SlotsComponent.GetSlotPrimaryItem` _returnvalue_2)))
        (bind _value_2 (`self.HowMuchCanBeInserted`))
        (bind (_success_2 _amountactuallyremoved_2) (`self.RemoveFluid` _asliquid_tank_parent_2 (`KismetMathLibrary.FMin` _value_2 0.05)))
        (`self.AddFluid` "dirty_water" _amountactuallyremoved_2)))))

(event `self.ReceiveBeginPlay`
  (set `self.FluidMax` 40.0)
  (`parent.ReceiveBeginPlay`)
  (`|ExecutionSequence`
    (:`then_0`
      (`KismetSystemLibrary.K2_SetTimerDelegate` (delegate `CheckTank`) 0.1 true))
    (:`then_1`
      (setmembers `TooltipWidgetDisplayData` :`StructRef` (`TooltipComponent.DefaultDisplayData` (`self.TooltipComponent`)) :`InteractionPrompts` (`|MakeArray` (make `InteractionPromptEntryData` "Use" "None" "None" 0.0 false "Drink +5")))
      (add `self.UV` (delegate `Update Visuals Event`))
      (`self.UV`))))

(event `Update Visuals Event`
  (`PoseableMeshComponent.SetBoneLocationByName` (`self.FluidMesh`) "Root_001" (`KismetMathLibrary.MakeVector` 0.0 0.0 (`KismetMathLibrary.Lerp` 109.230087 285.39801 (/ (`self.FluidCurrent`) (`self.FluidMax`)))) "ComponentSpace")
  (`self.UpdateDescription`))

(event `InputAction|Use`
  (params (Key :type "Key Structure"))
  (:`Pressed`
    (bind _returnvalue (`GameplayStatics.GetActorOfClass` "/Game/Mods/Yzch/AstroVitals/HungerManager.HungerManager_C"))
    (bind (_success _amountactuallyremoved) (`self.RemoveFluid` 5.0))
    (`/Game/Mods/Yzch/AstroVitals/HungerManager.OnDrink` _returnvalue _amountactuallyremoved)
    (`AstroStatics.PlaySound` "/Game/Mods/Yzch/AstroVitals/Gluck.Gluck")))

(fn `UserConstructionScript`
  (`parent.UserConstructionScript`))