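; FoodCan_BP is a food can item in the AstroVitals mod that stores units of a single food type and their accumulated hunger value.
; CanAddFood accepts food only when the can is below capacity and either has no type yet or already holds the same type.
; AddFood sets the type, increments the count and adds the value, then rebuilds the tooltip showing food name, fill level and hunger gain, which also initializes on BeginPlay.
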(event `self.ReceiveBeginPlay`
  (`self.UpdateDescription`))

(fn `AddFood`
  (params (Food :type "ItemType Class Reference") (AddFoodValue :type "Float (double-precision)"))
  (set `self.FoodType` Food)
  (bind _output_get (set `self.CurrentFood` (+ (stale _output_get) 1)))
  (bind _output_get_2 (set `self.FoodValue` (+ (stale _output_get_2) AddFoodValue)))
  (`self.UpdateDescription`))

(fn `CanAddFood`
  (params (Food :type "ItemType Class Reference"))
  (returns (Can :type Boolean))
  (bind _foodtype (`self.FoodType`))
  (return (and (or (== Food _foodtype) (== _foodtype null)) (< (`self.CurrentFood`) (`self.MaxFood`)))))

(fn `UpdateDescription`
  (bind _foodtype (`self.FoodType`))
  (setmembers `TooltipWidgetDisplayData` :`StructRef` (`TooltipComponent.DefaultDisplayData` (`self.TooltipComponent`)) :`Description` (`KismetTextLibrary.Conv_StringToText` (`KismetStringLibrary.Concat_StrStr` "Food: " (select `bool` (== _foodtype null) :`false` (`KismetTextLibrary.Conv_TextToString` (`ControlSymbol.Name` (`AstroPlayStatics.GetControlSymbolDefault` _foodtype)))) " \nContent: " (`KismetStringLibrary.Conv_IntToString` (`self.CurrentFood`)) "/" (`KismetStringLibrary.Conv_IntToString` (`self.MaxFood`)) " \nFood (+" (`KismetStringLibrary.Conv_IntToString` (`KismetMathLibrary.Round` (`self.FoodValue`))) " hunger)"))))

(fn `UserConstructionScript`
  (`parent.UserConstructionScript`))