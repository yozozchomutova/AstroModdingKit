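; Small drinkable liquid bottle item for the AstroVitals mod, built on a parent fluid container with a fixed small capacity.
; On BeginPlay it sets capacity, adds a Use tooltip prompt and binds an update-visuals event that refreshes the description.
; Pressing Use passes the current fluid amount to the HungerManager's OnDrink, plays a gulp sound and empties the tank.
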(event `self.ReceiveBeginPlay`
  (set `self.FluidMax` 8.0)
  (`parent.ReceiveBeginPlay`)
  (setmembers `TooltipWidgetDisplayData` :`StructRef` (`TooltipComponent.DefaultDisplayData` (`self.TooltipComponent`)) :`InteractionPrompts` (`|MakeArray` (make `InteractionPromptEntryData` "Use" "None" "None" 0.0 false "Drink")))
  (add `self.UV` (delegate `Update Visuals Event`))
  (`self.UV`))

(event `Update Visuals Event`
  (`self.UpdateDescription`))

(event `InputAction|Use`
  (params (Key :type "Key Structure"))
  (:`Pressed`
    (bind _returnvalue (`GameplayStatics.GetActorOfClass` "/Game/Mods/Yzch/AstroVitals/HungerManager.HungerManager_C"))
    (`/Game/Mods/Yzch/AstroVitals/HungerManager.OnDrink` _returnvalue (`self.FluidCurrent`))
    (`AstroStatics.PlaySound` "/Game/Mods/Yzch/AstroVitals/Gluck.Gluck")
    (`self.EmptyTank`)))

(fn `UserConstructionScript`
  (`parent.UserConstructionScript`))