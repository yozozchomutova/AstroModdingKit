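; Conveyor belt node for the LogisticsPlus mod, a pass-through point with one belt input and one belt output.
; The construction script cross-links the two attach components and assigns their touch colliders, plus the indicator and rail for the output.
; Moving the node or changing its motion state unlinks both connections through the ConveyorLinkSystem actor.
; Movable updates pass both attach points to UpdateMovableFunc.
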(event `UpdateMovable_`
  (`self.UpdateMovableFunc` (`|MakeArray` (`self.ConveyorBeltAttachOut`)) (`|MakeArray` (`self.ConveyorBeltAttachIn`))))

(event `self.ReceiveBeginPlay`
  (add `self.UpdateMovable` (delegate `UpdateMovable_`))
  (`parent.ReceiveBeginPlay`)
  (add `PhysicalItem.OnMoved` (delegate `OnMoved_Event_0`))
  (add `PhysicalItem.OnMotionStateChanged` (delegate `ONMotio`)))

(event `ONMotio`
  (bind _conveyorbeltattachin (`self.ConveyorBeltAttachIn`))
  (bind _conveyorbeltattachout (`self.ConveyorBeltAttachOut`))
  (bind _linkedattachout (`/Game/Mods/Yzch/LogisticsPlus/Components/ConveyorBeltAttachIn.LinkedAttachOut` _conveyorbeltattachin))
  (bind _linkedattachin (`/Game/Mods/Yzch/LogisticsPlus/Components/ConveyorBeltAttachOut.LinkedAttachIn` _conveyorbeltattachout))
  (bind _returnvalue (`GameplayStatics.GetActorOfClass` "/Game/Mods/Yzch/LogisticsPlus/Components/ConveyorLinkSystem.ConveyorLinkSystem_C" :!label _label))
  (`|ExecutionSequence`
    (:`then_0`
      (if (!= null _linkedattachout)
        (`/Game/Mods/Yzch/LogisticsPlus/Components/ConveyorLinkSystem.Unlink` _returnvalue _conveyorbeltattachin _linkedattachout)))
    (:`then_1`
      (if (!= null _linkedattachin)
        (`/Game/Mods/Yzch/LogisticsPlus/Components/ConveyorLinkSystem.Unlink` _returnvalue _linkedattachin _conveyorbeltattachout)))))

(event `OnMoved_Event_0`
  (params (FromTool :type Boolean))
  (goto _label))

(fn `GetBodySlotLegacy`
  (returns (ReturnValue :type "ChildSlotComponent Object Reference"))
  (return (`self.BodySlot`)))

(fn `UserConstructionScript`
  (`|ExecutionSequence`
    (:`then_0`
      (set `/Game/Mods/Yzch/LogisticsPlus/Components/ConveyorBeltAttachOut.TouchCollider` (`self.AttachOut`) (`self.ConveyorBeltAttachOut`))
      (set `/Game/Mods/Yzch/LogisticsPlus/Components/ConveyorBeltAttachOut.Indicator` (`self.Indicator`) (`self.ConveyorBeltAttachOut`))
      (set `/Game/Mods/Yzch/LogisticsPlus/Components/ConveyorBeltAttachOut.Rail` (`self.Rail`) (`self.ConveyorBeltAttachOut`))
      (set `/Game/Mods/Yzch/LogisticsPlus/Components/ConveyorBeltAttachIn.ContinueAttachOut` (`self.ConveyorBeltAttachOut`) (`self.ConveyorBeltAttachIn`))
      (set `/Game/Mods/Yzch/LogisticsPlus/Components/ConveyorBeltAttachOut.ContinueAttachIn` (`self.ConveyorBeltAttachIn`) (`self.ConveyorBeltAttachOut`)))
    (:`then_1`
      (set `/Game/Mods/Yzch/LogisticsPlus/Components/ConveyorBeltAttachIn.TouchCollider` (`self.AttachIn`) (`self.ConveyorBeltAttachIn`)))))