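; Conveyor belt end piece for the LogisticsPlus mod, with a single input attach point and no outputs.
; Construction assigns the attach point's touch collider, and BeginPlay binds handlers for movable updates, moves and motion state changes.
; Moves and motion changes unlink any linked upstream output through the ConveyorLinkSystem actor, while movable updates pass the input to UpdateMovableFunc.
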(event `UpdateMovable_`
  (`self.UpdateMovableFunc` (`|MakeArray`) (`|MakeArray` (`self.ConveyorBeltAttachIn`))))

(event `self.ReceiveBeginPlay`
  (add `self.UpdateMovable` (delegate `UpdateMovable_`))
  (`parent.ReceiveBeginPlay`)
  (add `PhysicalItem.OnMoved` (delegate `OnMoved_Event_0`))
  (add `PhysicalItem.OnMotionStateChanged` (delegate `ONMotio`)))

(event `ONMotio`
  (bind _conveyorbeltattachin (`self.ConveyorBeltAttachIn`))
  (bind _linkedattachout (`/Game/Mods/Yzch/LogisticsPlus/Components/ConveyorBeltAttachIn.LinkedAttachOut` _conveyorbeltattachin))
  (bind _returnvalue (`GameplayStatics.GetActorOfClass` "/Game/Mods/Yzch/LogisticsPlus/Components/ConveyorLinkSystem.ConveyorLinkSystem_C" :!label _label))
  (if (!= null _linkedattachout)
    (`/Game/Mods/Yzch/LogisticsPlus/Components/ConveyorLinkSystem.Unlink` _returnvalue _conveyorbeltattachin _linkedattachout)))

(event `OnMoved_Event_0`
  (params (FromTool :type Boolean))
  (goto _label))

(fn `GetBodySlotLegacy`
  (returns (ReturnValue :type "ChildSlotComponent Object Reference"))
  (return (`self.BodySlot`)))

(fn `UserConstructionScript`
  (set `/Game/Mods/Yzch/LogisticsPlus/Components/ConveyorBeltAttachIn.TouchCollider` (`self.AttachIn`) (`self.ConveyorBeltAttachIn`)))