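; Conveyor belt platform for the LogisticsPlus mod that rides along linked conveyor belts until it is picked up.
; Each tick it steps a fixed distance, not scaled by delta time, toward the attach-out's current arm position, taking that arm's rotation with a direction-dependent roll offset.
; At segment ends it hops to the linked continuation or reverses if none exists.
; Physics is off while attached; pickup detaches it and re-enables physics.
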(event `self.ReceiveBeginPlay`
  (add `self.OnPickedUpFromWorld` (delegate `PickedUp`))
  (if (!= null (`self.ConveyourBeltAttachOut`))
    (`PrimitiveComponent.SetSimulatePhysics` (`self.StaticMeshComponent`) false)))

(event `PickedUp` :!signature `self.OnPickedUpFromWorld`
  (params (PhysicalMovement :type Boolean))
  (set `self.ConveyourBeltAttachOut` null)
  (`PrimitiveComponent.SetSimulatePhysics` (`self.StaticMeshComponent`) true))

(event `self.ReceiveTick`
  (params (DeltaSeconds :type "Float (single-precision)"))
  (bind _returnvalue (`SceneComponent.K2_GetComponentLocation` (`self.StaticMeshComponent`)))
  (bind _continueattachin (`/Game/Mods/Yzch/LogisticsPlus/Components/ConveyorBeltAttachOut.ContinueAttachIn` (`self.ConveyourBeltAttachOut`)))
  (bind _continueattachout (`/Game/Mods/Yzch/LogisticsPlus/Components/ConveyorBeltAttachIn.ContinueAttachOut` (`/Game/Mods/Yzch/LogisticsPlus/Components/ConveyorBeltAttachOut.LinkedAttachIn` (`self.ConveyourBeltAttachOut`))))
  (if (!= null (`self.ConveyourBeltAttachOut`))
    (`SceneComponent.K2_SetWorldLocation` (`self.StaticMeshComponent`) (+ (* (`KismetMathLibrary.Normal` (- (`|GetArrayItem` (`/Game/Mods/Yzch/LogisticsPlus/Components/ConveyorBeltAttachOut.ArmPosition` (`self.ConveyourBeltAttachOut`)) (`self.Arm`)) _returnvalue) 0.001) 8.0) _returnvalue) false false)
    (`SceneComponent.K2_SetWorldRotation` (`self.StaticMeshComponent`) (`KismetMathLibrary.MakeRotator` (+ (.roll (`|GetArrayItem` (`/Game/Mods/Yzch/LogisticsPlus/Components/ConveyorBeltAttachOut.ArmRotation` (`self.ConveyourBeltAttachOut`)) (`self.Arm`))) (select `bool` (`self.Returns`) :`false` -90.0 :`true` 90.0 :!type "Float (single-precision)")) (.pitch (`|GetArrayItem` (`/Game/Mods/Yzch/LogisticsPlus/Components/ConveyorBeltAttachOut.ArmRotation` (`self.ConveyourBeltAttachOut`)) (`self.Arm`))) (.yaw (`|GetArrayItem` (`/Game/Mods/Yzch/LogisticsPlus/Components/ConveyorBeltAttachOut.ArmRotation` (`self.ConveyourBeltAttachOut`)) (`self.Arm`)))) false false)
    (if (<= (`KismetMathLibrary.Vector_Distance` (`|GetArrayItem` (`/Game/Mods/Yzch/LogisticsPlus/Components/ConveyorBeltAttachOut.ArmPosition` (`self.ConveyourBeltAttachOut`)) (`self.Arm`)) (`SceneComponent.K2_GetComponentLocation` (`self.StaticMeshComponent`))) 10.0)
      (if (`self.Returns`)
        (bind _output_get (set `self.Arm` (+ (`self.Arm`) -1)))
        (if (<= _output_get -1)
          (if (!= null _continueattachin)
            (set `self.Arm` 13)
            (set `self.ConveyourBeltAttachOut` (`/Game/Mods/Yzch/LogisticsPlus/Components/ConveyorBeltAttachIn.LinkedAttachOut` _continueattachin))
            (else
              (set `self.Returns` false)
              (set `self.Arm` 0))))
        (else
          (set `self.Arm` (+ (`self.Arm`) 1))
          (if (>= (`self.Arm`) 14)
            (if (!= _continueattachout null)
              (set `self.Arm` 0)
              (set `self.ConveyourBeltAttachOut` _continueattachout)
              (else
                (set `self.Returns` true)
                (set `self.Arm` (- (`self.Arm`) 2))))))))))

(fn `GetBodySlotLegacy`
  (returns (ReturnValue :type "ChildSlotComponent Object Reference"))
  (return (`self.BodySlot`)))

(fn `UserConstructionScript`)