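; Start piece of the LogisticsPlus conveyor belt, providing a single outgoing attach point and a slot that feeds platforms onto the belt.
; A platform placed in the slot receives the attach-out and a reset arm, then is released with physics simulation disabled.
; Moving the start, or the physical item it is slotted into, unlinks the outgoing connection through ConveyorLinkSystem.
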(event `On Platform Item Placed`
  (params (Item :type "PhysicalItem Object Reference"))
  (bind _asconveyor_belt_platform_bp (cast `/Game/Mods/Yzch/LogisticsPlus/ConveyorBeltPlatform_BP` Item))
  (set `/Game/Mods/Yzch/LogisticsPlus/ConveyorBeltPlatform_BP.ConveyourBeltAttachOut` (`self.ConveyorBeltAttachOut`) _asconveyor_belt_platform_bp)
  (set `/Game/Mods/Yzch/LogisticsPlus/ConveyorBeltPlatform_BP.Arm` 0 _asconveyor_belt_platform_bp)
  (`SlotsComponent.ReleaseItem` (`ChildSlotComponent.MakeReference` (`self.PlatformSlot`)) _asconveyor_belt_platform_bp)
  (`PrimitiveComponent.SetSimulatePhysics` (`PhysicalItem.StaticMeshComponent` _asconveyor_belt_platform_bp) false))

(event `On Platform Item Released`
  (params (Item :type "PhysicalItem Object Reference")))

(event `UpdateMovable_`
  (`self.UpdateMovableFunc` (`|MakeArray` (`self.ConveyorBeltAttachOut`)) (`|MakeArray`)))

(event `On Slotted`
  (bind _asphysical_item (cast `PhysicalItem` (`ActorComponent.GetOwner` (`SlotsComponent.GetSlotOwner` (`self.CurrentSlot`)))))
  (bind _output_get (set `self.SlottedParent` _asphysical_item))
  (add `self.OnMoved` _output_get (delegate `Platform  Moved`)))

(event `On Unslotted` :!signature `self.OnReleasedFromSlot`
  (params (NewOwner :type Boolean))
  (remove `self.OnMoved` (`self.SlottedParent`) (delegate `Platform  Moved`)))

(event `self.ReceiveBeginPlay`
  (bind _returnvalue (`SlotsComponent.GetSlotDelegates` (`ChildSlotComponent.MakeReference` (`self.PlatformSlot`))))
  (add `self.UpdateMovable` (delegate `UpdateMovable_`))
  (`parent.ReceiveBeginPlay`)
  (add `SlotDelegates.OnSetItem` _returnvalue (delegate `On Platform Item Placed`))
  (add `SlotDelegates.OnReleaseItem` _returnvalue (delegate `On Platform Item Released`))
  (add `self.OnMoved` (delegate `OnMoved_Event_0`))
  (add `self.OnPlacedInSlot` (delegate `On Slotted`))
  (add `self.OnReleasedFromSlot` (delegate `On Unslotted`)))

(event `Platform  Moved` :!signature `self.OnMoved`
  (params (FromTool :type Boolean))
  (bind _conveyorbeltattachout (`self.ConveyorBeltAttachOut`))
  (bind _linkedattachin (`/Game/Mods/Yzch/LogisticsPlus/Components/ConveyorBeltAttachOut.LinkedAttachIn` _conveyorbeltattachout))
  (bind _returnvalue (`GameplayStatics.GetActorOfClass` "/Game/Mods/Yzch/LogisticsPlus/Components/ConveyorLinkSystem.ConveyorLinkSystem_C" :!label _label))
  (if (!= null _linkedattachin)
    (`/Game/Mods/Yzch/LogisticsPlus/Components/ConveyorLinkSystem.Unlink` _returnvalue _linkedattachin _conveyorbeltattachout)))

(event `OnMoved_Event_0` :!signature `self.OnMoved`
  (params (FromTool :type Boolean))
  (goto _label))

(fn `GetBodySlotLegacy`
  (returns (ReturnValue :type "ChildSlotComponent Object Reference"))
  (return (`self.BodySlot`)))

(fn `UserConstructionScript`
  (bind _conveyorbeltattachout (`self.ConveyorBeltAttachOut`))
  (set `/Game/Mods/Yzch/LogisticsPlus/Components/ConveyorBeltAttachOut.TouchCollider` (`self.AttachOut`) _conveyorbeltattachout)
  (set `/Game/Mods/Yzch/LogisticsPlus/Components/ConveyorBeltAttachOut.Indicator` (`self.Indicator`) _conveyorbeltattachout)
  (set `/Game/Mods/Yzch/LogisticsPlus/Components/ConveyorBeltAttachOut.Rail` (`self.Rail`) _conveyorbeltattachout))