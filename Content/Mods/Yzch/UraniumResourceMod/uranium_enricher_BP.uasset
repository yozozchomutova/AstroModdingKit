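; Uranium enricher machine that converts Uranite from an input slot into Uranium and Uranium Waste.
; Tick keeps partially filled items in both output slots, draining Uranite and filling them until either is full.
; Per-tick rates and animation speed scale with the power component's load-to-output ratio, without delta time.
; Outputs become clickable only when full; slot delegates track insertion and removal, and a depleted input shows a Uranite request indicator.
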(event `OnRelease EnrichedU Slot`
  (params (Item :type "PhysicalItem Object Reference"))
  (`SlotsComponent.SetSlotClickable` (`ChildSlotComponent.MakeReference` (`self.EnrichedUSlot`)))
  (set `self.Uranium235` null))

(event `self.ReceiveTick`
  (params (DeltaSeconds :type "Float (single-precision)"))
  (bind _powercomponent (`self.PowerComponent`))
  (bind _returnvalue (`ChildSlotComponent.MakeReference` (`self.WasteSlot`)))
  (bind _returnvalue_2 (`ChildSlotComponent.MakeReference` (`self.EnrichedUSlot`)))
  (bind _itemcomponent (`PhysicalItem.ItemComponent` (`self.UraniteItem`)))
  (bind _itemcomponent_2 (`PhysicalItem.ItemComponent` (`self.Uranium235`)))
  (bind _itemcomponent_3 (`PhysicalItem.ItemComponent` (`self.Uranium238`)))
  (bind _returnvalue_3 (/ (`KismetMathLibrary.Abs` (`PowerComponent.NetActualLoad` _powercomponent)) (`KismetMathLibrary.Abs` (`PowerComponent.NetPowerOutput` _powercomponent))))
  (bind _returnvalue_4 (< (`ItemComponent.GetFullness` (`PhysicalItem.ItemComponent` (`self.Uranium238`))) 1.0))
  (bind _returnvalue_5 (< (`ItemComponent.GetFullness` (`PhysicalItem.ItemComponent` (`self.Uranium235`))) 1.0))
  (if (== null (`self.Uranium235`))
    (`SlotsComponent.SpawnItemTypeInSlot` _returnvalue_2 "/Game/Mods/Yzch/UraniumResourceMod/Uranium.Uranium_C")
    (set `self.Uranium235` (`SlotsComponent.GetSlotItem` _returnvalue_2)))
  (if (== null (`self.Uranium238`))
    (`SlotsComponent.SpawnItemTypeInSlot` _returnvalue "/Game/Mods/Yzch/UraniumResourceMod/UraniumWaste.UraniumWaste_C")
    (set `self.Uranium238` (`SlotsComponent.GetSlotItem` _returnvalue)))
  (`SlotsComponent.SetSlotClickable` (`ChildSlotComponent.MakeReference` (`self.EnrichedUSlot`)) (not _returnvalue_5))
  (`SlotsComponent.SetSlotClickable` (`ChildSlotComponent.MakeReference` (`self.WasteSlot`)) (not _returnvalue_4))
  (if (and _returnvalue_5 _returnvalue_4 (!= (`self.UraniteItem`) null))
    (`SkeletalMeshComponent.SetPlayRate` (`self.SkeletalMesh`) (`self.animPlayRate`))
    (`|ExecutionSequence`
      (:`then_0`
        (`ItemComponent.SetAmountUsingFullness` _itemcomponent (- (`ItemComponent.GetFullness` _itemcomponent) (`KismetMathLibrary.Lerp` 0.0 0.025 _returnvalue_3)) false)
        (if (<= (`ItemComponent.GetFullness` (`PhysicalItem.ItemComponent` (`self.UraniteItem`))) 0.0)
          (`SlotsComponent.DestroySlotItem` (`ChildSlotComponent.MakeReference` (`self.InputSlot`)))
          (set `self.UraniteItem` null)
          (set `self.animPlayRate` 0.0)
          (`SkeletalMeshComponent.SetPlayRate` (`self.SkeletalMesh`) (`self.animPlayRate`))
          (`SlotsComponent.SlotPushIndicatorItemTypes` (`ChildSlotComponent.MakeReference` (`self.InputSlot`)) 1 (make `SlotIndicatorDefinition` "/Game/Mods/Yzch/UraniumResourceMod/Uranite.Uranite_C") :!label _label)))
      (:`then_1`
        (`ItemComponent.SetAmountUsingFullness` _itemcomponent_2 (+ (`ItemComponent.GetFullness` _itemcomponent_2) (`KismetMathLibrary.Lerp` 0.0 0.0042 _returnvalue_3)) false))
      (:`then_2`
        (`ItemComponent.SetAmountUsingFullness` _itemcomponent_3 (+ (`ItemComponent.GetFullness` _itemcomponent_3) (`KismetMathLibrary.Lerp` 0.0 0.0125 _returnvalue_3)) false))
      (:`then_3`
        (set `self.animPlayRate` (* _returnvalue_3 2.0))))
    (else
      (bind _output_get (set `self.animPlayRate` 0.0))
      (`SkeletalMeshComponent.SetPlayRate` (`self.SkeletalMesh`) _output_get))))

(event `OnRelease Waste Slot`
  (params (Item :type "PhysicalItem Object Reference"))
  (`SlotsComponent.SetSlotClickable` (`ChildSlotComponent.MakeReference` (`self.WasteSlot`)))
  (set `self.Uranium238` null))

(event `self.ReceiveBeginPlay`
  (bind _returnvalue (`ChildSlotComponent.MakeReference` (`self.WasteSlot`)))
  (bind _returnvalue_2 (`ChildSlotComponent.MakeReference` (`self.InputSlot`)))
  (bind _returnvalue_3 (`ChildSlotComponent.MakeReference` (`self.EnrichedUSlot`)))
  (`SkeletalMeshComponent.SetPlayRate` (`self.SkeletalMesh`) (`self.animPlayRate`))
  (add `SlotDelegates.OnSetItem` (`SlotsComponent.GetSlotDelegates` (`SlotsComponent.GetSlotOwner` _returnvalue_2) _returnvalue_2) (delegate `Input Item Slot`))
  (add `SlotDelegates.OnReleaseItem` (`SlotsComponent.GetSlotDelegates` (`SlotsComponent.GetSlotOwner` _returnvalue) _returnvalue) (delegate `OnRelease Waste Slot`))
  (add `SlotDelegates.OnReleaseItem` (`SlotsComponent.GetSlotDelegates` (`SlotsComponent.GetSlotOwner` _returnvalue_3) _returnvalue_3) (delegate `OnRelease EnrichedU Slot`))
  (goto _label))

(event `Input Item Slot`
  (params (Item :type "PhysicalItem Object Reference"))
  (set `self.UraniteItem` Item))

(fn `GetBodySlotLegacy`
  (returns (ReturnValue :type "ChildSlotComponent Object Reference"))
  (return (`self.BodySlot`)))

(fn `UserConstructionScript`)