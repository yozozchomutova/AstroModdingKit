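; Paint bucket item Blueprint that opens a painting UI and holds a limited number of uses.
; Pressing Use removes any existing PaintingUI widgets, then creates a new one linked back to the bucket; destroying the bucket also removes those widgets.
; It stores primary and secondary colors as vectors through UpdateColors.
; DecreaseUses counts down, refreshing the "Uses left" tooltip or destroying the bucket when none remain.
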(event `InputAction|Use`
  (params (Key :type "Key Structure"))
  (:`Pressed`
    (bind _foundwidgets (`WidgetBlueprintLibrary.GetAllWidgetsOfClass` "/Game/Mods/Yzch/Painting/PaintingUI.PaintingUI_C"))
    (for _array_element _foundwidgets
      (`/Game/Mods/Yzch/Painting/PaintingUI.DestroySelf` _array_element))
    (bind _returnvalue (`|GenericCreateObject` "/Game/Mods/Yzch/Painting/PaintingUI.PaintingUI_C" (`AstroPlayStatics.GetLocalPlayController`)))
    (bind _output_get (set `self.LinkedPaintingUI` _returnvalue))
    (set `/Game/Mods/Yzch/Painting/PaintingUI.PaintBucketParent` self _output_get)
    (`UserWidget.AddToViewport` (`self.LinkedPaintingUI`) 0)))

(event `self.ReceiveBeginPlay`
  (add `self.OnDestroyed` (delegate `OnDestroyed_Event_0`))
  (`self.UpdateDescription`))

(event `OnDestroyed_Event_0` :!signature `self.OnDestroyed`
  (params (DestroyedActor :type "Actor Object Reference"))
  (bind _foundwidgets (`WidgetBlueprintLibrary.GetAllWidgetsOfClass` "/Game/Mods/Yzch/Painting/PaintingUI.PaintingUI_C"))
  (for _array_element _foundwidgets
    (`/Game/Mods/Yzch/Painting/PaintingUI.DestroySelf` _array_element)))

(fn `DecreaseUses`
  (bind _result (`/Engine/EditorBlueprintResources/StandardMacros.DecrementInt` (`self.Uses`))
    (:`  `
      (set `self.Uses` _result)
      (if (<= (`self.Uses`) 0)
        (`self.K2_DestroyActor`)
        (else
          (`self.UpdateDescription`))))))

(fn `GetBodySlotLegacy`
  (returns (ReturnValue :type "ChildSlotComponent Object Reference"))
  (return (`self.Body Slot`)))

(fn `UpdateColors`
  (params (R_P :type "Float (double-precision)") (G_P :type "Float (double-precision)") (B_P :type "Float (double-precision)") (R_S :type "Float (double-precision)") (G_S :type "Float (double-precision)") (B_S :type "Float (double-precision)"))
  (set `self.PrimaryColor` (`KismetMathLibrary.MakeVector` R_P G_P B_P))
  (set `self.SecondaryColor` (`KismetMathLibrary.MakeVector` R_S G_S B_S)))

(fn `UpdateDescription`
  (bind (_interactionprompts _badgecolor _resourceobjectbadge _resourceobjectbadgebackground _description _title _subtitle _presentationstyle _animationdirection _custombadgesize _openastropediadeck _openastropediacard) (break `TooltipWidgetDisplayData` (`TooltipComponent.DefaultDisplayData` (`self.TooltipComponent`))))
  (set `TooltipComponent.DefaultDisplayData` (make `TooltipWidgetDisplayData` _interactionprompts _badgecolor _resourceobjectbadge _resourceobjectbadgebackground (`KismetTextLibrary.Conv_StringToText` (`KismetStringLibrary.Concat_StrStr` "Uses left: " (`KismetStringLibrary.Conv_IntToString` (`self.Uses`)))) _title _subtitle _presentationstyle _animationdirection _custombadgesize _openastropediadeck _openastropediacard) (`self.TooltipComponent`)))

(fn `UserConstructionScript`)