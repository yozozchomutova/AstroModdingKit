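; Example mod item that demonstrates a usable interaction by toggling global game speed, a placeholder effect meant for testing.
; Pressing Use checks the current time dilation and switches between normal and greatly accelerated time.
; Each switch sets the ClickableComponent's active use context to TurnOn or TurnOff, which updates the displayed action and any active tooltips.
; A legacy getter exposes the item's BodySlot.
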(event `InputAction|Use`
  (params (Key :type "Key Structure"))
  (:`Pressed`
    (if (> (`GameplayStatics.GetGlobalTimeDilation`) 1.5)
      ;[1 1 1] I only modify the time dilation for testing, you can change the functionality to whatever you like
      (`GameplayStatics.SetGlobalTimeDilation` 1.0)
      ;[1 1 1] The SetActiveUseContext method allows you to change what displays as the use action and automatically refreshes active tooltips if necessary
      (`ClickableComponent.SetActiveUseContext` (`self.ClickableComponent`) "UC_TurnOn")
      (else
        (`GameplayStatics.SetGlobalTimeDilation` 10.0)
        (`ClickableComponent.SetActiveUseContext` (`self.ClickableComponent`) "UC_TurnOff")))))

(fn `GetBodySlotLegacy`
  (returns (ReturnValue :type "ChildSlotComponent Object Reference"))
  (return (`self.BodySlot`)))

(fn `UserConstructionScript`)